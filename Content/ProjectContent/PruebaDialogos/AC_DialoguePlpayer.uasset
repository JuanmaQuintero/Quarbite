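; Player-side dialogue component that lets the owning actor talk to NPCs in range.
; Owner overlaps cache an actor's DIalogueActivator, and ending an overlap with any actor that has a component clears it.
; Pressing E opens a DIalogue_Box widget fed by the activator's data table, enabling the cursor and blocking move and look.
; Left clicks are forwarded to the widget, and StopDialogue restores game-only input and removes it.
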(event `self.ReceiveBeginPlay`
  (bind _returnvalue (`self.GetOwner`))
  (add `Actor.OnActorBeginOverlap` _returnvalue (delegate `Overlap`))
  (add `Actor.OnActorEndOverlap` _returnvalue (delegate `EndOverlap`)))

(event `Overlap`
  (params (OverlappedActor :type "Actor Object Reference") (OtherActor :type "Actor Object Reference"))
  (bind _returnvalue (`Actor.GetComponentByClass` OtherActor "/Game/ProjectContent/PruebaDialogos/DIalogueActivator.DIalogueActivator_C"))
  (`/Engine/EditorBlueprintResources/StandardMacros.IsValid` _returnvalue
    (:`Is Valid`
      (set `self.NPC in area` _returnvalue))))

(event `EndOverlap`
  (params (OverlappedActor :type "Actor Object Reference") (OtherActor :type "Actor Object Reference"))
  (`/Engine/EditorBlueprintResources/StandardMacros.IsValid` (`Actor.GetComponentByClass` OtherActor "/Script/Engine.ActorComponent")
    (:`Is Valid`
      (set `self.NPC in area` null))))

(event `Key|E`
  (params (Key :type "Key Structure"))
  (bind _npc_in_area (`self.NPC in area`))
  (:`Pressed`
    (`/Engine/EditorBlueprintResources/StandardMacros.IsValid` _npc_in_area
      (:`Is Valid`
        (`self.Start DIalogue` (`/Game/ProjectContent/PruebaDialogos/DIalogueActivator.Datatable` _npc_in_area) _npc_in_area)))))

(event `Key|LeftMouseButton`
  (params (Key :type "Key Structure"))
  (bind _dialogue_ref (`self.Dialogue ref`))
  (:`Pressed`
    (`/Engine/EditorBlueprintResources/StandardMacros.IsValid` _dialogue_ref
      (:`Is Valid`
        (`/Game/ProjectContent/PruebaDialogos/DIalogue_Box.Mouse pressed` _dialogue_ref)))))

(event `Start DIalogue`
  (params (`NPC DT` :type "DataTable Object Reference") (Activator :type "/Game/ProjectContent/PruebaDialogos/DIalogueActivator Object Reference"))
  (bind _returnvalue (`GameplayStatics.GetPlayerController` 0))
  (if (not (`self.In dialogue`))
    (set `self.In dialogue` true)
    (set `PlayerController.bShowMouseCursor` true _returnvalue)
    (`Controller.SetIgnoreMoveInput` _returnvalue true)
    (`Controller.SetIgnoreLookInput` _returnvalue true)
    (`WidgetBlueprintLibrary.SetInputMode_GameAndUIEx` _returnvalue null "DoNotLock" true true)
    (bind _returnvalue_2 (`|CreateWidget` "/Game/ProjectContent/PruebaDialogos/DIalogue_Box.DIalogue_Box_C"))
    (bind _output_get (set `self.Dialogue ref` _returnvalue_2))
    (`UserWidget.AddToViewport` _output_get 0)
    (`/Game/ProjectContent/Interfaces/I_Interact.Iniciate Dialogue` _returnvalue_2 self `NPC DT` Activator)))

(event `Stop Dialogue`
  (bind _returnvalue (`GameplayStatics.GetPlayerController` 0))
  (set `self.In dialogue` false)
  (set `PlayerController.bShowMouseCursor` false _returnvalue)
  (`Controller.SetIgnoreMoveInput` _returnvalue false)
  (`Controller.SetIgnoreLookInput` _returnvalue false)
  (`WidgetBlueprintLibrary.SetInputMode_GameOnly` _returnvalue)
  (`Widget.RemoveFromParent` (`self.Dialogue ref`)))