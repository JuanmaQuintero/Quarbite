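; NPC Blueprint that follows the player character through AI navigation.
; On BeginPlay it caches the BP_MainCharacter reference and issues an AI MoveTo targeting that actor, stopping within an acceptance radius.
; Each successful move calls MoveTowardsPlayer again to keep the follow loop running, while a failed move has no retry.
; Tick refreshes the stored player position fed to the Destination input, alongside the target actor.
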(event `self.ReceiveBeginPlay`
  (`self.Move Towards Player`))

(event `self.ReceiveTick`
  (params (DeltaSeconds :type "Float (single-precision)"))
  (`self.Get Player Position`))

(event `Move Towards Player`
  (bind _asbp_main_character (cast `/Game/ProjectContent/BluePrints/Character/BP_MainCharacter` (`GameplayStatics.GetPlayerCharacter` 0)))
  (bind _output_get (set `self.Player ref` _asbp_main_character))
  (`|AIMoveTo` self (`self.Player POS`) _output_get 250.0
    (:`OnSuccess`
      (`self.Move Towards Player`))))

(event `Get Player Position`
  (set `self.Player POS` (`self.K2_GetActorLocation` (`self.Player ref`))))

(fn `UserConstructionScript`)