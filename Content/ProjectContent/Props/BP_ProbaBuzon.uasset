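; BP_ProbaBuzon is an interactable mailbox prop, apparently a test, whose slot piece (BocaBuzon) swings open and closed.
; Each Interaction event toggles IsOpened and plays or reverses the Abrir timeline, ignoring input while it is still playing.
; The timeline's track scales TargetDegrees and adds OriginalDegrees to set the piece's relative pitch.
; BeginPlay caches the player character, though these graphs never use it, and the Interact function is empty.
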(event `self.ReceiveBeginPlay`
  ; Begin Play
  (bind _asbp_main_character (cast `/Game/ProjectContent/BluePrints/Character/BP_MainCharacter` (`GameplayStatics.GetPlayerCharacter` 0)))
  (set `self.Character Ref` _asbp_main_character)
  (set `self.IsOpened` false))

(event `/Game/ProjectContent/Interfaces/I_Interact.Interaction`
  (params (Interactor :type "Character Object Reference"))
  ; Interaction
  (`KismetSystemLibrary.PrintString` "Interactuar")
  (if (not (`TimelineComponent.IsPlaying` (`self.Abrir`)))
    (if (not (`self.IsOpened`))
      (set `self.IsOpened` true)
      (bind (_direction _newtrack_0) (`Timeline|Abrir` :!via `PlayFromStart` :!label _label)
        (:`Update`
          (set `self.New Track 0` _newtrack_0)
          (`SceneComponent.K2_SetRelativeRotation` (`self.BocaBuzon`) (`KismetMathLibrary.MakeRotator` 0.0 (+ (* _newtrack_0 (`self.TargetDegrees`)) (`self.OriginalDegrees`))) false false)))
      (else
        (set `self.IsOpened` false)
        (goto _label :!via `ReverseFromEnd`)))))

(fn `Interact`
  (params (Interactor :type "Character Object Reference"))
  (return))

(fn `UserConstructionScript`)