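; BP_SafeBox is a keypad safe puzzle that opens when the player enters a hard-coded five-digit combination.
; Interaction blends the camera to the safe and puts BP_MainCharacter into puzzle mode.
; Clickable keys build or erase the entry, and Enter counts position matches against the solution.
; Success turns two lights green and chains wheel and door timelines, while pickup on E is only a debug print gated by PuertaAbierta.
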(event `self.ReceiveBeginPlay`
  (set `self.solution` (`|MakeArray` 2 2 6 6 2))
  (bind _asbp_main_character (cast `/Game/ProjectContent/BluePrints/Character/BP_MainCharacter` (`GameplayStatics.GetPlayerPawn` 0)))
  (set `self.As BP Main Character` _asbp_main_character))

(event `Animacion de abrir`
  (bind (_direction _newtrack_0) (`Timeline|MoveWheel`)
    (:`Update`
      (`SceneComponent.K2_SetRelativeRotation` (`self.wheel`) (`KismetMathLibrary.MakeRotator` (* _newtrack_0 180.0)) false false))
    (:`Finished`
      (bind (_direction_2 _newtrack_0_2) (`Timeline|Open Door`)
        (:`Update`
          (`SceneComponent.K2_SetRelativeRotation` (`self.tape`) (`KismetMathLibrary.MakeRotator` 0.0 0.0 (* _newtrack_0_2 -75.0)) false false))
        (:`Finished`
          (set `self.puertaAbierta` false))))))

(event `/Game/ProjectContent/Interfaces/I_Interact.Interaction`
  (params (Interactor :type "Character Object Reference") (ItemToPut :type "/Game/ProjectContent/BluePrints/BP_InteractionItem Object Reference"))
  (`PlayerController.SetViewTargetWithBlend` (`GameplayStatics.GetPlayerController` 0) self 1.0 "VTBlend_Linear" 0.0 false)
  (`/Game/ProjectContent/BluePrints/Character/BP_MainCharacter.goPuzleMode` (`self.As BP Main Character`)))

(event `Key|E`
  (params (Key :type "Key Structure"))
  (:`Pressed`
    (if (`self.puertaAbierta`)
      (`KismetSystemLibrary.PrintString` "Coger pieza"))))

(event `self.1.OnClicked`
  (params (TouchedComponent :type "PrimitiveComponent Object Reference") (ButtonPressed :type "Key Structure"))
  (`self.addNumber` 1))

(event `self.2.OnClicked`
  (params (TouchedComponent :type "PrimitiveComponent Object Reference") (ButtonPressed :type "Key Structure"))
  (`self.addNumber` 2))

(event `self.3.OnClicked`
  (params (TouchedComponent :type "PrimitiveComponent Object Reference") (ButtonPressed :type "Key Structure"))
  (`self.addNumber` 3))

(event `self.4.OnClicked`
  (params (TouchedComponent :type "PrimitiveComponent Object Reference") (ButtonPressed :type "Key Structure"))
  (`self.addNumber` 4))

(event `self.5.OnClicked`
  (params (TouchedComponent :type "PrimitiveComponent Object Reference") (ButtonPressed :type "Key Structure"))
  (`self.addNumber` 5))

(event `self.6.OnClicked`
  (params (TouchedComponent :type "PrimitiveComponent Object Reference") (ButtonPressed :type "Key Structure"))
  (`self.addNumber` 6))

(event `self.7.OnClicked`
  (params (TouchedComponent :type "PrimitiveComponent Object Reference") (ButtonPressed :type "Key Structure"))
  (`self.addNumber` 7))

(event `self.8.OnClicked`
  (params (TouchedComponent :type "PrimitiveComponent Object Reference") (ButtonPressed :type "Key Structure"))
  (`self.addNumber` 8))

(event `self.9.OnClicked`
  (params (TouchedComponent :type "PrimitiveComponent Object Reference") (ButtonPressed :type "Key Structure"))
  (`self.addNumber` 9))

(event `self.erease.OnClicked`
  (params (TouchedComponent :type "PrimitiveComponent Object Reference") (ButtonPressed :type "Key Structure"))
  (`KismetArrayLibrary.Array_Clear` (`self.combination`)))

(event `self.0.OnClicked`
  (params (TouchedComponent :type "PrimitiveComponent Object Reference") (ButtonPressed :type "Key Structure"))
  (`self.addNumber` 0))

(event `self.enter.OnClicked`
  (params (TouchedComponent :type "PrimitiveComponent Object Reference") (ButtonPressed :type "Key Structure"))
  (`self.ValidateConbination`))

(fn `addNumber`
  (params (Number :type Integer))
  (`KismetArrayLibrary.Array_Add` (`self.combination`) Number)
  (`KismetSystemLibrary.PrintString` (`KismetStringLibrary.Conv_IntToString` Number)))

(fn `UserConstructionScript`)

(fn `ValidateConbination`
  (for (_array_element _array_index) (`self.combination`)
    (if (== _array_element (`|GetArrayItem` (`self.solution`) _array_index))
      (`/Engine/EditorBlueprintResources/StandardMacros.IncrementInt` (`self.aciertos`))))
  (if (== (- (`self.aciertos`) 1) (`KismetArrayLibrary.Array_LastIndex` (`self.solution`)))
    (`KismetSystemLibrary.PrintString` "completado")
    (`self.Animacion de abrir`)
    (`KismetArrayLibrary.Array_Clear` (`self.combination`))
    (set `self.aciertos` 0)
    (`PrimitiveComponent.SetMaterial` (`self.luz1`) 0 "/Game/ProjectContent/Props/Pruebas/Fusibles/M_GreenLight.M_GreenLight")
    (`PrimitiveComponent.SetMaterial` (`self.luz2`) 0 "/Game/ProjectContent/Props/Pruebas/Fusibles/M_GreenLight.M_GreenLight")
    (else
      (`KismetSystemLibrary.PrintString` "no es la clave")
      (`KismetArrayLibrary.Array_Clear` (`self.combination`))
      (set `self.aciertos` 0))))