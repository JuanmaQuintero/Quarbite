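; BP_InteractionItem is a pickup item actor configured from its row in DT_Items, looked up by Name.
; The construction script applies that row's mesh and collision box size.
; Interaction calls DoPick, which disables box collision and sends the row data and a self reference to player pawn 0 via PickUpItemMessage.
; HighLightItem applies an overlay material, but StopHighLightItem is empty, so nothing clears it here.
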(event `/Game/ProjectContent/Interfaces/I_Interact.Interaction`
  (params (Interactor :type "Character Object Reference") (ItemToPut :type "/Game/ProjectContent/BluePrints/BP_InteractionItem Object Reference"))
  (`KismetSystemLibrary.PrintString` "Picked")
  (`self.DoPick`))

(event `/Game/ProjectContent/Interfaces/I_Interact.HighLightItem`
  (`MeshComponent.SetOverlayMaterial` (`self.Item`) "/Game/ProjectContent/Material/M_HighLight2_Inst.M_HighLight2_Inst"))

(event `/Game/ProjectContent/Interfaces/I_Interact.StopHighLightItem`)

(fn `DoPick`
  (bind _returnvalue (`|GetDataTableRow` "/Game/ProjectContent/Inventory/DT_Items.DT_Items" (`self.name`))
    (:`then`
      (`PrimitiveComponent.SetCollisionEnabled` (`self.Box`) "NoCollision")
      (message `/Game/ProjectContent/Interfaces/I_Interact.PickUpItem` (`GameplayStatics.GetPlayerPawn` 0) _returnvalue self))))

(fn `UserConstructionScript`
  (bind _returnvalue (`|GetDataTableRow` "/Game/ProjectContent/Inventory/DT_Items.DT_Items" (`self.name`))
    (:`then`
      (bind (_name _description _mesh _type _collisionsize) (break `/Game/ProjectContent/Inventory/S_Item` _returnvalue))
      (`StaticMeshComponent.SetStaticMesh` (`self.Item`) _mesh)
      (`BoxComponent.SetBoxExtent` (`self.Box`) _collisionsize true))))