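; BP_PanicManager controls a panic screen effect by overwriting the settings of a PostProcessVolume found at BeginPlay.
; PanicOn and PanicOff play and reverse the AddPanic timeline, scaled to PanicDuration, but its intensity output is multiplied by zero.
; FullPanicTemporary sets high intensity with manual exposure, then zeroes intensity after a delay.
; The RemovePanic timeline is never run.
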(event `self.ReceiveBeginPlay`
  (`self.UpdatePanicDuration` (`self.PanicDuration`))
  (bind _returnvalue (`GameplayStatics.GetActorOfClass` "/Script/Engine.PostProcessVolume"))
  (set `self.PostProcess` _returnvalue))

(event `PanicOn`
  (bind (_direction _newtrack_0) (`Timeline|AddPanic` :!label _label)
    (:`Update`
      (set `PostProcessVolume.Settings` (make `PostProcessSettings` :`AutoExposureMethod` "AEM_Manual" :`SceneFringeIntensity` (* _newtrack_0 0.0) :`AutoExposureBias` 6.0) (`self.PostProcess`)))))

(event `PanicOff`
  (goto _label :!via `Reverse`))

(event `FullPanicTemporary`
  (set `PostProcessVolume.Settings` (make `PostProcessSettings` :`AutoExposureMethod` "AEM_Manual" :`SceneFringeIntensity` 10.0 :`AutoExposureBias` 10.0) (`self.PostProcess`))
  (`KismetSystemLibrary.Delay` 4.0)
  (set `PostProcessVolume.Settings` (make `PostProcessSettings` :`AutoExposureMethod` "AEM_Manual" :`AutoExposureBias` 10.0) (`self.PostProcess`)))

(fn `UpdatePanicDuration`
  (params (PanicDurationSecs :type "Float (double-precision)"))
  (`TimelineComponent.SetPlayRate` (`self.AddPanic`) (/ 1.0 PanicDurationSecs)))

(fn `UserConstructionScript`)