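; Fuse box puzzle: its lid opens only with the LB key tag, and interacting blends the view to the box and puts the player in puzzle mode.
; Clicking each of seven fuses rotates it on a timeline and appends its number to the combination.
; The main fuse then checks that order against Solution, spawning the garage trigger on a match or resetting the fuses and combination otherwise.
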(event `self.ReceiveBeginPlay`
  (bind _asbp_main_character (cast `/Game/ProjectContent/BluePrints/Character/BP_MainCharacter` (`GameplayStatics.GetPlayerPawn` 0)))
  (set `self.MainCharacter` _asbp_main_character)
  (`self.EnableInput` (`GameplayStatics.GetPlayerController` 0))
  (bind _returnvalue (`GameplayStatics.GetActorOfClass` "/Game/ProjectContent/BluePrints/Character/BP_UIManager.BP_UIManager_C"))
  (set `self.UIManager` _returnvalue)
  (set `self.Fusibles` (`|MakeArray` (`self.Fusible1`) (`self.Fusible2`) (`self.Fusible3`) (`self.Fusible4`) (`self.Fusible5`) (`self.Fusiblr6`) (`self.Fusible7`) :!type "SceneComponent Object Reference")))

(event `/Game/ProjectContent/Interfaces/I_Interact.Interaction`
  (params (Interactor :type "Character Object Reference") (ItemToPut :type "/Game/ProjectContent/BluePrints/Items/BP_InteractionItem Object Reference") (ComponentHit :type "ActorComponent Object Reference"))
  (`self.OpenTape`)
  (`PlayerController.SetViewTargetWithBlend` (`GameplayStatics.GetPlayerController` 0) self 0.5 "VTBlend_Linear" 0.0 false)
  (`/Game/ProjectContent/BluePrints/Character/BP_MainCharacter.goPuzleMode` (`self.MainCharacter`))
  (set `self.isInPuzle` true))

(event `EnhancedInput|/Game/ProjectContent/Inputs/InputsPuzle/IA_GoOutOfPuzzle`
  (params (ActionValue :type Boolean) (ElapsedSeconds :type "Float (double-precision)") (TriggeredSeconds :type "Float (double-precision)") (InputAction :type "InputAction Object Reference" :default "/Game/ProjectContent/Inputs/InputsPuzle/IA_GoOutOfPuzzle.IA_GoOutOfPuzzle"))
  (:`Started`
    (if (`self.isInPuzle`)
      (`PlayerController.SetViewTargetWithBlend` (`GameplayStatics.GetPlayerController` 0) (`GameplayStatics.GetPlayerPawn` 0) 0.5 "VTBlend_Linear" 0.0 false)
      (`/Game/ProjectContent/BluePrints/Character/BP_MainCharacter.goNormalMode` (`self.MainCharacter`))
      (`self.CloseTape`))))

(event `self.Fusible1.OnClicked`
  (params (TouchedComponent :type "PrimitiveComponent Object Reference") (ButtonPressed :type "Key Structure"))
  ; Switches Event
  (`self.SwitchState` TouchedComponent 1))

(event `self.Fusible2.OnClicked`
  (params (TouchedComponent :type "PrimitiveComponent Object Reference") (ButtonPressed :type "Key Structure"))
  ; Switches Event
  (`self.SwitchState` TouchedComponent 2))

(event `self.Fusible4.OnClicked`
  (params (TouchedComponent :type "PrimitiveComponent Object Reference") (ButtonPressed :type "Key Structure"))
  ; Switches Event
  (`self.SwitchState` TouchedComponent 4))

(event `self.Fusible3.OnClicked`
  (params (TouchedComponent :type "PrimitiveComponent Object Reference") (ButtonPressed :type "Key Structure"))
  ; Switches Event
  (`self.SwitchState` TouchedComponent 3))

(event `SwitchState`
  (params (FusibleToRotate :type "SceneComponent Object Reference") (Fusible :type Integer))
  (if (not (`TimelineComponent.IsPlaying` (`self.Timeline`)))
    (`KismetArrayLibrary.Array_Add` (`self.Combination`) Fusible)
    (bind (_direction _newtrack_0) (`Timeline|Timeline` :!via `PlayFromStart`)
      (:`Update`
        (`SceneComponent.K2_SetRelativeRotation` FusibleToRotate (`KismetMathLibrary.MakeRotator` (* _newtrack_0 -90.0)) false false)))))

(event `self.Fusible5.OnClicked`
  (params (TouchedComponent :type "PrimitiveComponent Object Reference") (ButtonPressed :type "Key Structure"))
  ; Switches Event
  (`self.SwitchState` TouchedComponent 5))

(event `self.Fusiblr6.OnClicked`
  (params (TouchedComponent :type "PrimitiveComponent Object Reference") (ButtonPressed :type "Key Structure"))
  ; Switches Event
  (`self.SwitchState` TouchedComponent 6))

(event `self.fusiblePrincipal.OnClicked`
  (params (TouchedComponent :type "PrimitiveComponent Object Reference") (ButtonPressed :type "Key Structure"))
  ; Switches Event
  (`self.subirPrincipal`))

(event `self.Fusible7.OnClicked`
  (params (TouchedComponent :type "PrimitiveComponent Object Reference") (ButtonPressed :type "Key Structure"))
  ; Switches Event
  (`self.SwitchState` TouchedComponent 7))

(event `BajarTodos`
  (bind _array_element (`/Game/ProjectContent/PruebaDialogos/DialogueMacros.ForEachLoopWithDelay` (`self.Fusibles`) 0.1)
    (:`LoopBody`
      (bind (_direction _newtrack_0) (`Timeline|Timeline_0` :!via `PlayFromStart`)
        (:`Update`
          (`KismetSystemLibrary.PrintString` (`KismetStringLibrary.Conv_DoubleToString` _newtrack_0))
          (`SceneComponent.K2_SetRelativeRotation` _array_element (`KismetMathLibrary.MakeRotator` (* _newtrack_0 -90.0)) false false))))
    (:`Completed`
      (`KismetArrayLibrary.Array_Clear` (`self.Combination`)))))

(event `/Game/ProjectContent/Interfaces/I_Interact.HighLightItem`
  (`MeshComponent.SetOverlayMaterial` (`self.tape`) "/Game/ProjectContent/Material/Ligths/M_HighLight2_Inst.M_HighLight2_Inst"))

(event `OpenTape`
  (bind _uimanager (`self.UIManager`))
  (if (`BlueprintGameplayTagLibrary.HasTag` (`/Game/ProjectContent/BluePrints/Character/BP_MainCharacter.EstatesTags` (`self.MainCharacter`)) (struct :`TagName` "Player.HasLBKey"))
    (`self.StopHighLightItem`)
    (bind (_direction _newtrack_0) (`Timeline|OpenTapeTimeline` :!label _label)
      (:`Update`
        (`SceneComponent.K2_SetRelativeRotation` (`self.tape`) (`KismetMathLibrary.MakeRotator` (* _newtrack_0 -140.0)) false false)))
    (else
      (`/Game/ProjectContent/BluePrints/Character/BP_UIManager.Show HelpUI` _uimanager)
      (set `TextBlock.Text` "Bloquejat amb clau." (`/Game/ProjectContent/UI/W_Help.TextToChange` (`/Game/ProjectContent/BluePrints/Character/BP_UIManager.Help` _uimanager))))))

(event `CloseTape`
  (goto _label :!via `Reverse`))

(event `/Game/ProjectContent/Interfaces/I_Interact.StopHighLightItem`
  (`MeshComponent.SetOverlayMaterial` (`self.tape`) null))

(event `subirPrincipal`
  (set `self.principalUp?` true)
  (bind (_direction _newtrack_0) (`Timeline|UP/DOWN` :!label _label_2)
    (:`Update`
      (`SceneComponent.K2_SetRelativeRotation` (`self.fusiblePrincipal`) (`KismetMathLibrary.MakeRotator` (* _newtrack_0 -90.0)) false false))
    (:`Finished`
      (`self.CheckSolution`))))

(event `bajarPrincipal`
  (set `self.principalUp?` false)
  (goto _label_2 :!via `Reverse`))

(fn `CheckSolution`
  (set `self.SwitchHits` 0)
  (if (`self.principalUp?`)
    (for (_array_element _array_index) (`self.Solution`)
      (if (== _array_element (`|GetArrayItem` (`self.Combination`) _array_index))
        (`/Engine/EditorBlueprintResources/StandardMacros.IncrementInt` (`self.SwitchHits`))))
    (if (== (`self.SwitchHits`) 7)
      (`KismetSystemLibrary.PrintString` "Completado")
      (`|SpawnActorFromClass` "/Game/ProjectContent/BluePrints/Triggers/Trigger_Garage.Trigger_Garage_C" (`KismetMathLibrary.MakeTransform` (1851.378284 -409.312588 39.817927)) "Undefined" "MultiplyWithRoot" null null)
      (else
        (`KismetSystemLibrary.PrintString` "Intenta de nuevo")
        (`self.BajarTodos`)
        (`self.bajarPrincipal`)))))

(fn `UserConstructionScript`)