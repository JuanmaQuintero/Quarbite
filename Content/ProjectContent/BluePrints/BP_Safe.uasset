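; BP_Safe is an interactable safe that puts the player into a puzzle view.
; On BeginPlay it caches the player's BP_MainCharacter.
; Interaction blends the camera to the safe, enables mouse cursor and click input, disables character movement, hides the HUD and flags the puzzle as active.
; The puzzle is unfinished: the Cylinder click event is empty, its rotation node is unconnected, and no exit logic exists.
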(event `self.ReceiveBeginPlay`
  (bind _asbp_main_character (cast `/Game/ProjectContent/BluePrints/Character/BP_MainCharacter` (`GameplayStatics.GetPlayerPawn` 0)))
  (set `self.As BP Main Character` _asbp_main_character))

(event `/Game/ProjectContent/Interfaces/I_Interact.Interaction`
  (params (Interactor :type "Character Object Reference") (ItemToPut :type "/Game/ProjectContent/BluePrints/BP_InteractionItem Object Reference"))
  (bind _returnvalue (`GameplayStatics.GetPlayerController` 0))
  (`PlayerController.SetViewTargetWithBlend` _returnvalue self 0.5 "VTBlend_Linear" 0.0 false)
  (set `PlayerController.bEnableClickEvents` true _returnvalue)
  (set `PlayerController.bShowMouseCursor` true _returnvalue)
  (`WidgetBlueprintLibrary.SetInputMode_GameAndUIEx` _returnvalue null "DoNotLock" false)
  (`CharacterMovementComponent.DisableMovement` (`Character.CharacterMovement` (`self.As BP Main Character`)))
  (`/Game/ProjectContent/BluePrints/Character/BP_MainCharacter.HideHUD` (`self.As BP Main Character`))
  (set `self.isInPuzle` true))

(event `self.Cylinder.OnClicked`
  (params (TouchedComponent :type "PrimitiveComponent Object Reference") (ButtonPressed :type "Key Structure")))

(fn `UserConstructionScript`)