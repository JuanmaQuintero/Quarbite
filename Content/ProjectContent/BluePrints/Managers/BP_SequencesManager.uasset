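; BP_SequencesManager is a manager actor that plays the game's main and final cinematics and handles what follows them.
; Two events create Level Sequence players for those cinematics; the final one waits a fixed delay, then opens the main menu level.
; PlayerAfterSequence calls PostSequence on the player character and on a BP_NPC found in the level.
; The kitchen light event is an empty stub.
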(event `self.ReceiveBeginPlay`)

(event `PlayMainSequence`
  (bind (_outactor _returnvalue) (`LevelSequencePlayer.CreateLevelSequencePlayer` "/Game/ProjectContent/Cinematics/MainCinematic.MainCinematic"))
  (`MovieSceneSequencePlayer.Play` _returnvalue))

(event `PlayFinalSequence`
  (bind (_outactor _returnvalue) (`LevelSequencePlayer.CreateLevelSequencePlayer` "/Game/ProjectContent/Cinematics/FinalCinematic.FinalCinematic"))
  (`MovieSceneSequencePlayer.Play` _returnvalue)
  (`KismetSystemLibrary.Delay` 34.0)
  (`GameplayStatics.OpenLevelBySoftObjectPtr` "/Game/ProjectContent/Levels/MainMenu.MainMenu"))

(event `PlayerAfterSequence`
  (bind _asbp_main_character (cast `/Game/ProjectContent/BluePrints/Character/BP_MainCharacter` (`GameplayStatics.GetPlayerPawn` 0)))
  (`/Game/ProjectContent/BluePrints/Character/BP_MainCharacter.PostSequence` _asbp_main_character)
  (bind _returnvalue (`GameplayStatics.GetActorOfClass` "/Game/ProjectContent/BluePrints/NPC/BP_NPC.BP_NPC_C"))
  (`/Game/ProjectContent/BluePrints/NPC/BP_NPC.PostSequence` _returnvalue))

(event `encederLuzCocina`)

(fn `UserConstructionScript`)