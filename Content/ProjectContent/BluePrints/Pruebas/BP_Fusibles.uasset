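; Fuse box puzzle actor: interacting opens the lid, blends the view to the box and puts the player in puzzle mode.
; Clicking one of seven fuses toggles its Ups entry through a shared timeline that rotates it and blocks overlapping clicks.
; The main fuse raises, then CheckSolution compares Ups with the solution, lighting a spotlight or dropping the fuse back.
; A separate Solution event colours two indicator lights from fuse pairs before checking.
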(event `self.ReceiveBeginPlay`
  (set `self.As BP Flash Light` null)
  (bind _asbp_main_character (cast `/Game/ProjectContent/BluePrints/Character/BP_MainCharacter` (`GameplayStatics.GetPlayerPawn` 0)))
  (set `self.MainCharacter` _asbp_main_character)
  (`self.EnableInput` (`GameplayStatics.GetPlayerController` 0))
  (set `self.light01_Material` (`PrimitiveComponent.GetMaterial` (`self.Light1`) 0))
  (set `self.light02_Material` (`PrimitiveComponent.GetMaterial` (`self.Light2`) 0))
  (bind _returnvalue (`GameplayStatics.GetActorOfClass` "/Game/ProjectContent/BluePrints/Character/BP_UIManager.BP_UIManager_C"))
  (set `self.UIManager` _returnvalue))

(event `/Game/ProjectContent/Interfaces/I_Interact.Interaction`
  (params (Interactor :type "Character Object Reference") (ItemToPut :type "/Game/ProjectContent/BluePrints/BP_InteractionItem Object Reference"))
  (`self.OpenTape`)
  (`LightComponent.SetIntensity` (`Light.LightComponent` (`self.PuzleLight`)) 1.2)
  (`PlayerController.SetViewTargetWithBlend` (`GameplayStatics.GetPlayerController` 0) self 0.5 "VTBlend_Linear" 0.0 false)
  (`/Game/ProjectContent/BluePrints/Character/BP_MainCharacter.goPuzleMode` (`self.MainCharacter`)))

(event `self.Fusible0.OnClicked`
  (params (TouchedComponent :type "PrimitiveComponent Object Reference") (ButtonPressed :type "Key Structure"))
  ; Switches Event
  (`self.SwitchState` TouchedComponent))

(event `self.Fusible1.OnClicked`
  (params (TouchedComponent :type "PrimitiveComponent Object Reference") (ButtonPressed :type "Key Structure"))
  ; Switches Event
  (`self.SwitchState` TouchedComponent 1))

(event `self.Fusible3.OnClicked`
  (params (TouchedComponent :type "PrimitiveComponent Object Reference") (ButtonPressed :type "Key Structure"))
  ; Switches Event
  (`self.SwitchState` TouchedComponent 3))

(event `self.Fusible2.OnClicked`
  (params (TouchedComponent :type "PrimitiveComponent Object Reference") (ButtonPressed :type "Key Structure"))
  ; Switches Event
  (`self.SwitchState` TouchedComponent 2))

(event `SwitchState`
  (params (FusibleToRotate :type "SceneComponent Object Reference") (Index :type Integer))
  (bind _ups (`self.Ups`))
  (if (not (`TimelineComponent.IsPlaying` (`self.Timeline`)))
    (`KismetArrayLibrary.Array_Set` _ups Index (not (`|GetArrayItem` _ups Index)))
    (if (`|GetArrayItem` (`self.Ups`) Index)
      (bind (_direction _newtrack_0) (`Timeline|Timeline` :!via `PlayFromStart` :!label _label)
        (:`Update`
          (`SceneComponent.K2_SetRelativeRotation` FusibleToRotate (`KismetMathLibrary.MakeRotator` (* _newtrack_0 -90.0)) false false)))
      (else
        (goto _label :!via `ReverseFromEnd`)))))

(event `self.Fusible4.OnClicked`
  (params (TouchedComponent :type "PrimitiveComponent Object Reference") (ButtonPressed :type "Key Structure"))
  ; Switches Event
  (`self.SwitchState` TouchedComponent 4))

(event `self.Fusible5.OnClicked`
  (params (TouchedComponent :type "PrimitiveComponent Object Reference") (ButtonPressed :type "Key Structure"))
  ; Switches Event
  (`self.SwitchState` TouchedComponent 5))

(event `self.fusiblePrincipal.OnClicked`
  (params (TouchedComponent :type "PrimitiveComponent Object Reference") (ButtonPressed :type "Key Structure"))
  ; Switches Event
  (`self.subirPrincipal`))

(event `self.Fusible6.OnClicked`
  (params (TouchedComponent :type "PrimitiveComponent Object Reference") (ButtonPressed :type "Key Structure"))
  ; Switches Event
  (`self.SwitchState` TouchedComponent 6))

(event `Solution`
  (bind _ups (`self.Ups`))
  (bind _ups_2 (`self.Ups`))
  (if (and (not (`|GetArrayItem` _ups_2)) (`|GetArrayItem` _ups_2 1))
    (`PrimitiveComponent.SetMaterial` (`self.Light1`) 0 "/Game/ProjectContent/Props/Pruebas/Fusibles/M_GreenLight.M_GreenLight")
    (else
      (`PrimitiveComponent.SetMaterial` (`self.Light1`) 0 "/Game/ProjectContent/Props/Pruebas/Fusibles/M_RedLight.M_RedLight")))
  (if (and (`|GetArrayItem` _ups 2) (not (`|GetArrayItem` _ups 3)))
    (`PrimitiveComponent.SetMaterial` (`self.Light2`) 0 "/Game/ProjectContent/Props/Pruebas/Fusibles/M_GreenLight.M_GreenLight")
    (else
      (`PrimitiveComponent.SetMaterial` (`self.Light2`) 0 "/Game/ProjectContent/Props/Pruebas/Fusibles/M_RedLight.M_RedLight")))
  (`self.CheckSolution`))

(event `/Game/ProjectContent/Interfaces/I_Interact.HighLightItem`
  (`MeshComponent.SetOverlayMaterial` (`self.tape`) "/Game/ProjectContent/Material/M_HighLight2_Inst.M_HighLight2_Inst"))

(event `OpenTape`
  (bind (_direction _newtrack_0) (`Timeline|Open`)
    (:`Update`
      (`SceneComponent.K2_SetRelativeRotation` (`self.tape`) (`KismetMathLibrary.MakeRotator` (* _newtrack_0 -140.0)) false false)
      (`self.StopHighLightItem`))))

(event `/Game/ProjectContent/Interfaces/I_Interact.StopHighLightItem`
  (`MeshComponent.SetOverlayMaterial` (`self.tape`) null))

(event `subirPrincipal`
  (bind (_direction _newtrack_0) (`Timeline|Timeline_0` :!label _label_2)
    (:`Update`
      (`SceneComponent.K2_SetRelativeRotation` (`self.fusiblePrincipal`) (`KismetMathLibrary.MakeRotator` (* _newtrack_0 -90.0)) false false))
    (:`Finished`
      (`self.CheckSolution`))))

(event `bajarPrincipal`
  (set `self.principalUp?` false)
  (goto _label_2 :!via `Reverse`))

(fn `CheckSolution`
  (set `self.principalUp?` true)
  (set `self.SwitchHits` 0)
  (if (`self.principalUp?`)
    (for (_array_element _array_index) (`self.solutionCombination`)
      (if (== _array_element (`|GetArrayItem` (`self.Ups`) _array_index))
        (`/Engine/EditorBlueprintResources/StandardMacros.IncrementInt` (`self.SwitchHits`))))
    (if (== (`self.SwitchHits`) (`KismetArrayLibrary.Array_Length` (`self.SolutionPuzle`)))
      (`KismetSystemLibrary.PrintString` "Completado")
      (`LightComponent.SetIntensity` (`SpotLight.SpotLightComponent` (`self.LightToTurnOn`)) 106.453766)
      (else
        (`KismetSystemLibrary.PrintString` "No yet!")
        (`self.bajarPrincipal`)))))

(fn `UserConstructionScript`)