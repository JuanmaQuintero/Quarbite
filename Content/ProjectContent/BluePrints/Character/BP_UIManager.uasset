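; BP_UIManager is a Blueprint that creates and holds the game's UI widgets: HUD, circles, menus, help, letters and death screen.
; On BeginPlay it creates and caches all six widgets, but adds only the HUD, stored as Dot, to the viewport.
; Custom events show and hide the help, letter and death widgets through AddToViewport and RemoveFromParent.
; The circles and menus widgets are only created and stored here, with no show or hide events.
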(event `self.ReceiveBeginPlay`
  ; Inicialización widgets
  (bind _returnvalue (`|CreateWidget` "/Game/ProjectContent/UI/W_HUD.W_HUD_C" (`GameplayStatics.GetPlayerController` 0)))
  (bind _output_get (set `self.Dot` _returnvalue))
  (`UserWidget.AddToViewport` _output_get 0)
  (bind _returnvalue_2 (`|CreateWidget` "/Game/ProjectContent/UI/W_Circles.W_Circles_C" (`GameplayStatics.GetPlayerController` 0)))
  (set `self.Circles` _returnvalue_2)
  (bind _returnvalue_3 (`|CreateWidget` "/Game/ProjectContent/UI/W_Menus.W_Menus_C"))
  (set `self.Menus` _returnvalue_3)
  (bind _returnvalue_4 (`|CreateWidget` "/Game/ProjectContent/UI/W_Help.W_Help_C"))
  (set `self.Help` _returnvalue_4)
  (bind _returnvalue_5 (`|CreateWidget` "/Game/ProjectContent/UI/W_Letters.W_Letters_C"))
  (set `self.Letters` _returnvalue_5)
  (bind _returnvalue_6 (`|CreateWidget` "/Game/ProjectContent/UI/UI_Death.UI_Death_C"))
  (set `self.Death` _returnvalue_6))

(event `Show HelpUI`
  (`UserWidget.AddToViewport` (`self.Help`) 0))

(event `Hide HelpUI`
  (`Widget.RemoveFromParent` (`self.Help`)))

(event `ShowDeath`
  (`UserWidget.AddToViewport` (`self.Death`) 0))

(event `ShowLetterContent`
  (`UserWidget.AddToViewport` (`self.Letters`) 0))

(event `HideLetterContent`
  (`Widget.RemoveFromParent` (`self.Letters`)))

(event `HideDeath`
  (`Widget.RemoveFromParent` (`self.Death`)))

(fn `UserConstructionScript`)