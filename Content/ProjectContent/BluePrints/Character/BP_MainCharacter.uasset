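; First-person player character that handles movement, look, walk camera shake, object interaction, item pickup and opening the pause menu.
; A short camera trace each tick switches the crosshair for I_Interact actors, and a matching trace on input sends InteractionMessage with the left-hand item.
; Pickups update the UIManager inventory, then attach to either hand or, for the key, set a gameplay tag.
; A held frame slows walking, and the light input triggers the right-hand item.
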(event `HeadBob`
  ; Head Movement
  (if (> (`KismetMathLibrary.VSize` (`self.GetVelocity`)) 0.0)
    (`PlayerController.ClientStartCameraShake` :`self` (`GameplayStatics.GetPlayerController` 0) :`Shake` "/Game/ProjectContent/BluePrints/Character/WalkShake.WalkShake_C")))

(event `self.ReceiveBeginPlay`
  ; Begin Play
  (bind _returnvalue (`GameplayStatics.GetActorOfClass` "/Game/ProjectContent/BluePrints/Character/BP_UIManager.BP_UIManager_C"))
  (set `self.UIManager` _returnvalue)
  (bind _asplayer_controller (cast `PlayerController` (`self.GetController`)))
  (`EnhancedInputSubsystemInterface.AddMappingContext` (pcsubsystem `EnhancedInputLocalPlayerSubsystem` _asplayer_controller) "/Game/ProjectContent/Inputs/IMC_Character.IMC_Character" 0 (struct)))

(event `ShowHUD`
  (bind _crosshair (`/Game/ProjectContent/UI/W_HUD.Crosshair` (`/Game/ProjectContent/BluePrints/Character/BP_UIManager.Dot` (`self.UIManager`))))
  ; Show HUD
  (`Widget.SetIsEnabled` _crosshair true)
  (`Widget.SetVisibility` _crosshair "Visible"))

(event `EnhancedInput|/Game/ProjectContent/Inputs/IA_MoveCharacter`
  (params (ActionValue :type "Vector2D Structure") (ElapsedSeconds :type "Float (double-precision)") (TriggeredSeconds :type "Float (double-precision)") (InputAction :type "InputAction Object Reference" :default "/Game/ProjectContent/Inputs/IA_MoveCharacter.IA_MoveCharacter"))
  ; Movement
  (:`Triggered`
    (`self.AddMovementInput` (`self.GetActorRightVector`) ActionValue_X)
    (`self.AddMovementInput` (`self.GetActorForwardVector`) ActionValue_Y)))

(event `HideHUD`
  (bind _crosshair (`/Game/ProjectContent/UI/W_HUD.Crosshair` (`/Game/ProjectContent/BluePrints/Character/BP_UIManager.Dot` (`self.UIManager`))))
  ; Hide HUD
  (`Widget.SetIsEnabled` _crosshair false)
  (`Widget.SetVisibility` _crosshair "Hidden"))

(event `EnhancedInput|/Game/ProjectContent/Inputs/IA_LookCharacter`
  (params (ActionValue :type "Vector2D Structure") (ElapsedSeconds :type "Float (double-precision)") (TriggeredSeconds :type "Float (double-precision)") (InputAction :type "InputAction Object Reference" :default "/Game/ProjectContent/Inputs/IA_LookCharacter.IA_LookCharacter"))
  ; Camera
  (:`Triggered`
    (`self.AddControllerYawInput` ActionValue_X)
    (`self.AddControllerPitchInput` ActionValue_Y)))

(event `/Game/ProjectContent/Interfaces/I_Interact.PickUpItem`
  (params (`Item Data` :type "/Game/ProjectContent/Inventory/S_Item Structure") (BP_Reference :type "/Game/ProjectContent/BluePrints/BP_InteractionItem Object Reference"))
  (bind (_name _description _mesh _type) (break `/Game/ProjectContent/Inventory/S_Item` `Item Data`))
  ; Inventory & Items to Hand
  (`KismetArrayLibrary.Array_Add` (`self.InventaryItems`) `Item Data`)
  (`/Game/ProjectContent/UI/W_Menus.RefreshInventory` (`/Game/ProjectContent/BluePrints/Character/BP_UIManager.Menus` (`self.UIManager`)))
  (if (`|EnumEquality` _type "NewEnumerator1")
    (set `self.InRightHand` BP_Reference)
    (if true
      (`self.K2_AttachToComponent` BP_Reference (`self.HandPoint`) " " "SnapToTarget" "SnapToTarget" "SnapToTarget" true)
      (`BlueprintGameplayTagLibrary.AddGameplayTag` (`self.EstatesTags`) (struct :`TagName` "Player.FlashLightOn")))
    (elif (`|EnumEquality` _type "NewEnumerator2")
      (bind _output_get (set `self.InLeftHand` BP_Reference))
      (`self.K2_AttachToComponent` _output_get (`self.HoldPoint`) " " "SnapToTarget" "SnapToTarget" "SnapToTarget" true)
      (set `self.HasFrame` true)
      (elif (`KismetTextLibrary.EqualEqual_TextText` (`.Name_9_C0CB730846DD33AA88A3E9B0BD212CF4` (break `/Game/ProjectContent/Inventory/S_Item` `Item Data`)) (`self.Key`))
        (`BlueprintGameplayTagLibrary.AddGameplayTag` (`self.EstatesTags`) (struct :`TagName` "Player.HasMainKey"))
        (`self.K2_DestroyActor` BP_Reference)
        (else
          (`self.K2_DestroyActor`))))))

(event `EnhancedInput|/Game/ProjectContent/Inputs/IA_Interact`
  (params (ActionValue :type Boolean) (ElapsedSeconds :type "Float (double-precision)") (TriggeredSeconds :type "Float (double-precision)") (InputAction :type "InputAction Object Reference" :default "/Game/ProjectContent/Inputs/IA_Interact.IA_Interact"))
  (bind _cameraplayer (`self.CameraPlayer`))
  (bind _returnvalue (`SceneComponent.K2_GetComponentLocation` _cameraplayer))
  ; Interact with interactuable objects
  (:`Started`
    (bind (_outhit _returnvalue_2) (`KismetSystemLibrary.LineTraceSingle` :`Start` _returnvalue :`End` (+ _returnvalue (* (`SceneComponent.GetForwardVector` _cameraplayer) 120.0)) :`TraceChannel` "TraceTypeQuery1" :`bTraceComplex` true :`DrawDebugType` "ForDuration"))
    (if _returnvalue_2
      (set `self.HitActor` (`.HitActor` (`GameplayStatics.BreakHitResult` _outhit)))
      (message `/Game/ProjectContent/Interfaces/I_Interact.Interaction` (`self.HitActor`) (`GameplayStatics.GetPlayerCharacter` 0) (`self.InLeftHand`))
      (`KismetSystemLibrary.PrintString` (`KismetSystemLibrary.GetDisplayName` null)))))

(event `self.ReceiveTick`
  (params (DeltaSeconds :type "Float (single-precision)"))
  (bind _cameraplayer (`self.CameraPlayer`))
  (bind _charactermovement (`self.CharacterMovement`))
  (bind _returnvalue (`SceneComponent.K2_GetComponentLocation` _cameraplayer))
  ; Event Tick
  (`self.HeadBob`)
  (if (`self.HasFrame`)
    (set `CharacterMovementComponent.MaxWalkSpeed` 80.0 _charactermovement)
    (else
      (set `CharacterMovementComponent.MaxWalkSpeed` 130.0 _charactermovement)))
  ; Change Cursor
  (bind (_outhit _returnvalue_2) (`KismetSystemLibrary.LineTraceSingle` _returnvalue (+ _returnvalue (* (`SceneComponent.GetForwardVector` _cameraplayer) 120.0)) "TraceTypeQuery1" true))
  (if _returnvalue_2
    (if (`KismetSystemLibrary.DoesImplementInterface` (`.HitActor` (`GameplayStatics.BreakHitResult` _outhit)) "/Game/ProjectContent/Interfaces/I_Interact.I_Interact_C")
      (`Image.SetBrushFromTexture` (`/Game/ProjectContent/UI/W_HUD.Crosshair` (`/Game/ProjectContent/BluePrints/Character/BP_UIManager.Dot` (`self.UIManager`))) "/Game/ProjectContent/UI/HandCrosshair.HandCrosshair" false)
      (else
        (`Image.SetBrushFromTexture` (`/Game/ProjectContent/UI/W_HUD.Crosshair` (`/Game/ProjectContent/BluePrints/Character/BP_UIManager.Dot` (`self.UIManager`))) "/Game/ProjectContent/UI/DotCrosshair.DotCrosshair" true :!label _label)))
    (else
      (goto _label))))

(event `EnhancedInput|/Game/ProjectContent/Inputs/IA_Light`
  (params (ActionValue :type Boolean) (ElapsedSeconds :type "Float (double-precision)") (TriggeredSeconds :type "Float (double-precision)") (InputAction :type "InputAction Object Reference" :default "/Game/ProjectContent/Inputs/IA_Light.IA_Light"))
  (bind _inrighthand (`self.InRightHand`))
  ; Turn On/Off
  (:`Started`
    (`/Engine/EditorBlueprintResources/StandardMacros.IsValid` _inrighthand
      (:`Is Valid`
        (`/Game/ProjectContent/Interfaces/I_Interact.HandInteraction` _inrighthand)))))

(event `EnhancedInput|/Game/ProjectContent/Inputs/IA_MenuPause`
  (params (ActionValue :type Boolean) (ElapsedSeconds :type "Float (double-precision)") (TriggeredSeconds :type "Float (double-precision)") (InputAction :type "InputAction Object Reference" :default "/Game/ProjectContent/Inputs/IA_MenuPause.IA_MenuPause"))
  (bind _returnvalue (`GameplayStatics.GetPlayerController` 0))
  (bind _menus (`/Game/ProjectContent/BluePrints/Character/BP_UIManager.Menus` (`self.UIManager`)))
  ; Menu
  (:`Started`
    (`UserWidget.AddToViewport` _menus 0)
    (set `PlayerController.bEnableClickEvents` true _returnvalue)
    (set `PlayerController.bShowMouseCursor` true _returnvalue)
    (`WidgetBlueprintLibrary.SetInputMode_UIOnlyEx` _returnvalue _menus)))

(fn `UserConstructionScript`)