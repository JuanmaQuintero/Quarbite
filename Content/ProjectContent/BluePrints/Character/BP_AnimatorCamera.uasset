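; BP_AnimatorCamera plays a scripted look-left camera turn (MirarIzquierda) on the player character at BeginPlay.
; It caches BP_MainCharacter, disables pawn control rotation on its CameraPlayer, and plays the Rotate timeline.
; Each update sets relative rotation from controller roll and pitch, with yaw as the sum of track value and control yaw, times 90.
; When the timeline finishes, pawn control rotation is re-enabled.
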(event `self.ReceiveBeginPlay`
  (bind _asbp_main_character (cast `/Game/ProjectContent/BluePrints/Character/BP_MainCharacter` (`GameplayStatics.GetPlayerPawn` 0)))
  (set `self.As BP Main Character` _asbp_main_character)
  (`self.Mirar Izquierda`))

(event `Mirar Izquierda`
  (set `CameraComponent.bUsePawnControlRotation` false (`/Game/ProjectContent/BluePrints/Character/BP_MainCharacter.CameraPlayer` (`self.As BP Main Character`)))
  (bind (_direction _newtrack_0) (`Timeline|Rotate` :!via `PlayFromStart`)
    (:`Update`
      (`SceneComponent.K2_SetRelativeRotation` (`/Game/ProjectContent/BluePrints/Character/BP_MainCharacter.CameraPlayer` (`self.As BP Main Character`)) (`KismetMathLibrary.MakeRotator` (.roll (`Controller.GetControlRotation` (`GameplayStatics.GetPlayerController` 0))) (.pitch (`Controller.GetControlRotation` (`GameplayStatics.GetPlayerController` 0))) (* (+ _newtrack_0 (.yaw (`Controller.GetControlRotation` (`GameplayStatics.GetPlayerController` 0)))) 90.0)) false false))
    (:`Finished`
      (set `CameraComponent.bUsePawnControlRotation` true (`/Game/ProjectContent/BluePrints/Character/BP_MainCharacter.CameraPlayer` (`self.As BP Main Character`))))))

(fn `UserConstructionScript`)