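; Interactable fuse box puzzle in which the player clicks four fuses to flip them and switch on a linked light.
; Interaction blends the view to the box, enables mouse clicks and freezes the character; the Back input restores normal play.
; Each click toggles a state and rotates the fuse through a shared Timeline.
; Solution then colors two indicator lights by hard-coded pairs, while CheckSolution compares all states against the solution array.
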(event `self.ReceiveBeginPlay`
  (bind _asbp_main_character (cast `/Game/ProjectContent/BluePrints/Character/BP_MainCharacter` (`GameplayStatics.GetPlayerPawn` 0)))
  (set `self.MainCharacter` _asbp_main_character)
  (`self.EnableInput` (`GameplayStatics.GetPlayerController` 0))
  (set `self.light01_Material` (`PrimitiveComponent.GetMaterial` (`self.Light1`) 0))
  (set `self.light02_Material` (`PrimitiveComponent.GetMaterial` (`self.Light2`) 0))
  (bind _returnvalue (`GameplayStatics.GetActorOfClass` "/Game/ProjectContent/BluePrints/Character/BP_UIManager.BP_UIManager_C"))
  (set `self.UIManager` _returnvalue))

(event `/Game/ProjectContent/Interfaces/I_Interact.Interaction`
  (params (Interactor :type "Character Object Reference") (ItemToPut :type "/Game/ProjectContent/BluePrints/BP_InteractionItem Object Reference"))
  (bind _returnvalue (`GameplayStatics.GetPlayerController` 0))
  (bind _maincharacter (`self.MainCharacter`))
  (`PlayerController.SetViewTargetWithBlend` _returnvalue self 0.5 "VTBlend_Linear" 0.0 false)
  (set `PlayerController.bEnableClickEvents` true _returnvalue)
  (set `PlayerController.bShowMouseCursor` true _returnvalue)
  (`WidgetBlueprintLibrary.SetInputMode_GameAndUIEx` _returnvalue null)
  (`CharacterMovementComponent.DisableMovement` (`Character.CharacterMovement` _maincharacter))
  (`/Game/ProjectContent/BluePrints/Character/BP_MainCharacter.HideHUD` _maincharacter)
  (`KismetSystemLibrary.PrintString` "Modo clicar"))

(event `EnhancedInput|/Game/ProjectContent/Inputs/IA_Back`
  (params (ActionValue :type Boolean) (ElapsedSeconds :type "Float (double-precision)") (TriggeredSeconds :type "Float (double-precision)") (InputAction :type "InputAction Object Reference" :default "/Game/ProjectContent/Inputs/IA_Back.IA_Back"))
  (bind _returnvalue (`GameplayStatics.GetPlayerController` 0))
  (bind _maincharacter (`self.MainCharacter`))
  (:`Started`
    (`PlayerController.SetViewTargetWithBlend` _returnvalue (`GameplayStatics.GetPlayerPawn` 0) 0.5 "VTBlend_Linear" 0.0 false)
    (set `PlayerController.bEnableClickEvents` false _returnvalue)
    (set `PlayerController.bShowMouseCursor` false _returnvalue)
    (`WidgetBlueprintLibrary.SetInputMode_GameOnly` _returnvalue)
    (`CharacterMovementComponent.SetMovementMode` (`Character.CharacterMovement` _maincharacter) "MOVE_Walking" 0)
    (`/Game/ProjectContent/BluePrints/Character/BP_MainCharacter.ShowHUD` _maincharacter)
    (`KismetSystemLibrary.PrintString` "Modo normal")
    (`Widget.RemoveFromParent` (`/Game/ProjectContent/BluePrints/Character/BP_UIManager.Menus` (`self.UIManager`)))))

(event `SwitchState`
  (params (FusibleToRotate :type "SceneComponent Object Reference") (Index :type Integer))
  (bind _ups (`self.Ups`))
  (if (not (`TimelineComponent.IsPlaying` (`self.Timeline`)))
    (`KismetArrayLibrary.Array_Set` _ups Index (not (`|GetArrayItem` _ups Index)))
    (if (`|GetArrayItem` (`self.Ups`) Index)
      (bind (_direction _newtrack_0) (`Timeline|Timeline` :!via `PlayFromStart` :!label _label)
        (:`Update`
          (`SceneComponent.K2_SetRelativeRotation` FusibleToRotate (`KismetMathLibrary.MakeRotator` (* _newtrack_0 90.0)) false false))
        (:`Finished`
          (`self.Solution`)))
      (else
        (goto _label :!via `ReverseFromEnd`)))))

(event `self.Fusible0.OnClicked`
  (params (TouchedComponent :type "PrimitiveComponent Object Reference") (ButtonPressed :type "Key Structure"))
  ; Switches Event
  (`KismetSystemLibrary.PrintString` "clicked")
  (`self.SwitchState` TouchedComponent))

(event `self.Fusible2.OnClicked`
  (params (TouchedComponent :type "PrimitiveComponent Object Reference") (ButtonPressed :type "Key Structure"))
  ; Switches Event
  (`self.SwitchState` TouchedComponent 2))

(event `self.Fusible3.OnClicked`
  (params (TouchedComponent :type "PrimitiveComponent Object Reference") (ButtonPressed :type "Key Structure"))
  ; Switches Event
  (`self.SwitchState` TouchedComponent 3))

(event `self.Fusible1.OnClicked`
  (params (TouchedComponent :type "PrimitiveComponent Object Reference") (ButtonPressed :type "Key Structure"))
  ; Switches Event
  (`self.SwitchState` TouchedComponent 1))

(event `Solution`
  (bind _ups (`self.Ups`))
  (bind _ups_2 (`self.Ups`))
  (if (and (not (`|GetArrayItem` _ups_2)) (`|GetArrayItem` _ups_2 1))
    (`PrimitiveComponent.SetMaterial` (`self.Light1`) 0 "/Game/ProjectContent/Props/Pruebas/Fusibles/M_GreenLight.M_GreenLight")
    (else
      (`PrimitiveComponent.SetMaterial` (`self.Light1`) 0 "/Game/ProjectContent/Props/Pruebas/Fusibles/M_RedLight.M_RedLight")))
  (if (and (`|GetArrayItem` _ups 2) (not (`|GetArrayItem` _ups 3)))
    (`PrimitiveComponent.SetMaterial` (`self.Light2`) 0 "/Game/ProjectContent/Props/Pruebas/Fusibles/M_GreenLight.M_GreenLight")
    (else
      (`PrimitiveComponent.SetMaterial` (`self.Light2`) 0 "/Game/ProjectContent/Props/Pruebas/Fusibles/M_RedLight.M_RedLight")))
  (`self.CheckSolution`))

(fn `CheckSolution`
  (set `self.SwitchHits` 0)
  (for (_array_element _array_index) (`self.SolutionPuzle`)
    (if (== _array_element (`|GetArrayItem` (`self.Ups`) _array_index))
      (`/Engine/EditorBlueprintResources/StandardMacros.IncrementInt` (`self.SwitchHits`))))
  (if (== (`self.SwitchHits`) (`KismetArrayLibrary.Array_Length` (`self.SolutionPuzle`)))
    (`KismetSystemLibrary.PrintString` "Completado")
    (`LightComponent.SetIntensity` (`PointLight.PointLightComponent` (`self.LightToTurnOn`)) 8000.0)
    (else
      (`KismetSystemLibrary.PrintString` "No yet!")
      (`LightComponent.SetIntensity` (`PointLight.PointLightComponent` (`self.LightToTurnOn`)) 0.0))))

(fn `UserConstructionScript`)