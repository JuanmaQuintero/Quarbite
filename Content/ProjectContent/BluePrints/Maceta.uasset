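; Maceta is an interactable prop Blueprint whose static mesh raises and lowers on alternating interactions and highlights on demand.
; BeginPlay caches the mesh's world position, and the Levantar timeline adds its track value to Z, applying the result as relative location.
; Interaction toggles IsUp to play or reverse the timeline, ignoring input while it runs.
; Highlight events set or clear an overlay material.
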(event `self.ReceiveBeginPlay`
  (bind (_returnvalue_x _returnvalue_y _returnvalue_z) (`KismetMathLibrary.BreakVector` (`SceneComponent.K2_GetComponentLocation` (`self.StaticMesh`))))
  (set `self.IsUp` false)
  (set `self.Z` _returnvalue_z)
  (set `self.X` _returnvalue_x)
  (set `self.Y` _returnvalue_y))

(event `/Game/ProjectContent/Interfaces/I_Interact.Interaction`
  (params (Interactor :type "Character Object Reference") (ItemToPut :type "/Game/ProjectContent/BluePrints/BP_InteractionItem Object Reference"))
  (if (not (`TimelineComponent.IsPlaying` (`self.Levantar`)))
    (if (not (`self.IsUp`))
      (set `self.IsUp` true)
      (bind (_direction _newtrack_0) (`Timeline|Levantar` :!via `PlayFromStart` :!label _label)
        (:`Update`
          (`SceneComponent.K2_SetRelativeLocation` (`self.StaticMesh`) (`KismetMathLibrary.MakeVector` (`self.X`) (`self.Y`) (+ (`self.Z`) _newtrack_0)) false false)))
      (else
        (set `self.IsUp` false)
        (goto _label :!via `ReverseFromEnd`)))))

(event `/Game/ProjectContent/Interfaces/I_Interact.HighLightItem`
  (`MeshComponent.SetOverlayMaterial` (`self.StaticMesh`) "/Game/ProjectContent/Materials/M_HighLight2_Inst.M_HighLight2_Inst"))

(event `/Game/ProjectContent/Interfaces/I_Interact.StopHighLightItem`
  (`MeshComponent.SetOverlayMaterial` (`self.StaticMesh`) null))

(fn `UserConstructionScript`)