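; BP_FrameSpot is a placement spot where the player can put a carried frame.
; On BeginPlay it caches the player pawn as BP_MainCharacter.
; Its Interaction event attaches a valid passed item to the spot's StaticMesh, snapping location, rotation and scale, then clears the character's HasFrame flag.
; Without a valid item it only prints a pick-up debug string ("recoger"), with no pickup logic.
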(event `self.ReceiveBeginPlay`
  (bind _asbp_main_character (cast `/Game/ProjectContent/BluePrints/Character/BP_MainCharacter` (`GameplayStatics.GetPlayerPawn` 0)))
  (set `self.As BP Main Character` _asbp_main_character))

(event `/Game/ProjectContent/Interfaces/I_Interact.Interaction`
  (params (Interactor :type "Character Object Reference") (ItemToPut :type "/Game/ProjectContent/BluePrints/BP_InteractionItem Object Reference"))
  (`/Engine/EditorBlueprintResources/StandardMacros.IsValid` ItemToPut
    (:`Is Valid`
      (`KismetSystemLibrary.PrintString` "Colocar")
      (`self.K2_AttachToComponent` ItemToPut (`self.StaticMesh`) " " "SnapToTarget" "SnapToTarget" "SnapToTarget" true)
      (set `/Game/ProjectContent/BluePrints/Character/BP_MainCharacter.HasFrame` false (`self.As BP Main Character`)))
    (:`Is Not Valid`
      (`KismetSystemLibrary.PrintString` "recoger"))))

(fn `UserConstructionScript`)