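; BP_OuijaTable is an interactable Ouija board puzzle where the player drags a pointer with the mouse.
; Interaction blends the view to the table, shows the cursor, disables character movement and hides the HUD.
; While the cone is held, Tick converts scaled mouse deltas, with swapped axes, into relative movement.
; On release, a timeline lerps the cone back to its original location, and clicks are ignored during that return.
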(event `self.ReceiveBeginPlay`
  (bind _asbp_main_character (cast `/Game/ProjectContent/BluePrints/Character/BP_MainCharacter` (`GameplayStatics.GetPlayerPawn` 0)))
  (set `self.As BP Main Character` _asbp_main_character)
  (set `self.OriginalLocationPunter` (`SceneComponent.RelativeLocation` (`self.Cone`))))

(event `/Game/ProjectContent/Interfaces/I_Interact.Interaction`
  (params (Interactor :type "Character Object Reference") (ItemToPut :type "/Game/ProjectContent/BluePrints/BP_InteractionItem Object Reference"))
  (bind _returnvalue (`GameplayStatics.GetPlayerController` 0))
  (bind _as_bp_main_character (`self.As BP Main Character`))
  (`PlayerController.SetViewTargetWithBlend` _returnvalue self 0.5 "VTBlend_Linear" 0.0 false)
  (set `PlayerController.bEnableClickEvents` true _returnvalue)
  (set `PlayerController.bShowMouseCursor` true _returnvalue)
  (`WidgetBlueprintLibrary.SetInputMode_GameAndUIEx` _returnvalue null "DoNotLock" false)
  (`CharacterMovementComponent.DisableMovement` (`Character.CharacterMovement` _as_bp_main_character))
  (`/Game/ProjectContent/BluePrints/Character/BP_MainCharacter.HideHUD` _as_bp_main_character)
  (set `self.isInPuzle` true))

(event `self.Cone.OnClicked`
  (params (TouchedComponent :type "PrimitiveComponent Object Reference") (ButtonPressed :type "Key Structure"))
  (bind (_locationx _locationy) (`PlayerController.GetMousePosition` (`GameplayStatics.GetPlayerController` 0)))
  (if (and (not (`TimelineComponent.IsPlaying` (`self.Timeline`))) (`self.isInPuzle`))
    (set `self.isDraging` true)
    (set `self.coneClicked` true)
    (`KismetSystemLibrary.PrintString` "Hello")
    (set `self.ClickedPostion` (`KismetMathLibrary.MakeVector2D` _locationx _locationy))))

(event `self.ReceiveTick`
  (params (DeltaSeconds :type "Float (single-precision)"))
  (bind (_locationx _locationy) (`PlayerController.GetMousePosition` (`GameplayStatics.GetPlayerController` 0)))
  (if (`self.isDraging`)
    (if (`self.coneClicked`)
      (bind (_y _x) (`self.CopyMousePosition`))
      (`SceneComponent.K2_AddRelativeLocation` (`self.Cone`) (`KismetMathLibrary.MakeVector` _y _x) false false)
      (set `self.ClickedPostion` (`KismetMathLibrary.MakeVector2D` _locationx _locationy)))))

(event `self.Cone.OnReleased`
  (params (TouchedComponent :type "PrimitiveComponent Object Reference") (ButtonReleased :type "Key Structure"))
  (bind (_relativelocation_x _relativelocation_y) (`KismetMathLibrary.BreakVector` (`SceneComponent.RelativeLocation` (`self.Cone`))))
  (`KismetSystemLibrary.PrintString` "He soltado el puntero")
  (set `self.isDraging` false)
  (bind (_y _x) (`self.CopyMousePosition`))
  (`SceneComponent.K2_AddRelativeLocation` (`self.Cone`) (`KismetMathLibrary.MakeVector` _y _x) false false)
  (set `self.vector2D` (`KismetMathLibrary.MakeVector2D` _relativelocation_x _relativelocation_y))
  (`self.PointerOuijaToOrigin`))

(event `PointerOuijaToOrigin`
  (bind _originallocationpunter (`self.OriginalLocationPunter`))
  (bind (_x _y) (`KismetMathLibrary.BreakVector2D` (`self.vector2D`)))
  (bind (_direction _newtrack_0) (`Timeline|Timeline` :!via `PlayFromStart`)
    (:`Update`
      (`SceneComponent.K2_SetRelativeLocation` (`self.Cone`) (`KismetMathLibrary.VLerp` (`KismetMathLibrary.MakeVector` _x _y (.z _originallocationpunter)) _originallocationpunter _newtrack_0) false false))))

(fn `CopyMousePosition`
  (returns (Y :type "Float (double-precision)") (X :type "Float (double-precision)"))
  (bind (_locationx _locationy) (`PlayerController.GetMousePosition` (`GameplayStatics.GetPlayerController` 0)))
  (bind (_x _y) (`KismetMathLibrary.BreakVector2D` (/ (- (`KismetMathLibrary.MakeVector2D` _locationx _locationy) (`self.ClickedPostion`)) 33.0)))
  (return (* _y -1.0) _x))

(fn `UserConstructionScript`)