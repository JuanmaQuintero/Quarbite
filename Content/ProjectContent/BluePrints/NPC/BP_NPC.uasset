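; BP_NPC is an interactable NPC and dialogue participant that starts its assigned dialogue on the interacting BP_MainCharacter.
; While patrolling, its StopArea overlaps tell AIC_NPCController when the player is near or away, and goPhone sends it to the phone.
; It plays the main sequence through BP_SequencesManager, and PostSequence moves it to the world origin.
; Participant getters supply name and gender, while condition, value and dialogue-event handlers are stubs.
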(event `self.ReceiveBeginPlay`
  (bind _returnvalue (`GameplayStatics.GetActorOfClass` "/Game/ProjectContent/BluePrints/Managers/BP_SequencesManager.BP_SequencesManager_C"))
  (set `self.NPC` _returnvalue))

(event `resetTakesPhone`
  (set `self.takesPhone` false))

(event `/Game/ProjectContent/Interfaces/I_Interact.Interaction`
  (params (Interactor :type "Character Object Reference") (ItemToPut :type "/Game/ProjectContent/BluePrints/Items/BP_InteractionItem Object Reference") (ComponentHit :type "ActorComponent Object Reference"))
  (bind _asbp_main_character (cast `/Game/ProjectContent/BluePrints/Character/BP_MainCharacter` Interactor))
  (`/Game/ProjectContent/BluePrints/Character/BP_MainCharacter.Start Dialogue` _asbp_main_character (`self.Asset to Start`)))

(event `self.StopArea.OnComponentBeginOverlap`
  (params (OverlappedComponent :type "PrimitiveComponent Object Reference") (OtherActor :type "Actor Object Reference") (OtherComp :type "PrimitiveComponent Object Reference") (OtherBodyIndex :type Integer) (bFromSweep :type Boolean) (SweepResult :type "HitResult Structure (by ref)"))
  (cast `/Game/ProjectContent/BluePrints/Character/BP_MainCharacter` OtherActor)
  (if (`self.isPatrolling`)
    (bind _asaic_npccontroller (cast `/Game/ProjectContent/BluePrints/NPC/AIC_NPCController` (`AIBlueprintHelperLibrary.GetAIController` self)))
    (`/Game/ProjectContent/BluePrints/NPC/AIC_NPCController.PlayerNear` _asaic_npccontroller)))

(event `self.StopArea.OnComponentEndOverlap`
  (params (OverlappedComponent :type "PrimitiveComponent Object Reference") (OtherActor :type "Actor Object Reference") (OtherComp :type "PrimitiveComponent Object Reference") (OtherBodyIndex :type Integer))
  (cast `/Game/ProjectContent/BluePrints/Character/BP_MainCharacter` OtherActor)
  (if (`self.isPatrolling`)
    (bind _asaic_npccontroller (cast `/Game/ProjectContent/BluePrints/NPC/AIC_NPCController` (`AIBlueprintHelperLibrary.GetAIController` self)))
    (`/Game/ProjectContent/BluePrints/NPC/AIC_NPCController.PlayerAway` _asaic_npccontroller)))

(event `goPhone`
  (bind _asaic_npccontroller (cast `/Game/ProjectContent/BluePrints/NPC/AIC_NPCController` (`AIBlueprintHelperLibrary.GetAIController` self)))
  (`/Game/ProjectContent/BluePrints/NPC/AIC_NPCController.GoToPhone` _asaic_npccontroller))

(event `MainSequence`
  (`/Game/ProjectContent/BluePrints/Managers/BP_SequencesManager.PlayMainSequence` (`self.NPC`)))

(event `PostSequence`
  (`self.K2_SetActorLocation` (0.0 0.0 0.0)))

(fn `CheckCondition`
  (params (Context :type "DlgContext Object Reference") (ConditionName :type Name))
  (returns (ReturnValue :type Boolean))
  (return false))

(fn `GetBoolValue`
  (params (ValueName :type Name))
  (returns (ReturnValue :type Boolean))
  (return false))

(fn `GetFloatValue`
  (params (ValueName :type Name))
  (returns (ReturnValue :type "Float (single-precision)"))
  (return 0.0))

(fn `GetIntValue`
  (params (ValueName :type Name))
  (returns (ReturnValue :type Integer))
  (return 0))

(fn `GetNameValue`
  (params (ValueName :type Name))
  (returns (ReturnValue :type Name))
  (return "None"))

(fn `GetParticipantDisplayName`
  (params (ActiveSpeaker :type Name))
  (returns (ReturnValue :type Text))
  (return (`self.DisplayName`)))

(fn `GetParticipantGender`
  (returns (ReturnValue :type "ETextGender Enum"))
  (return "Masculine"))

(fn `GetParticipantIcon`
  (params (ActiveSpeaker :type Name) (ActiveSpeakerState :type Name))
  (returns (ReturnValue :type "Texture2D Object Reference"))
  (return null))

(fn `GetParticipantName`
  (returns (ReturnValue :type Name))
  (return (`self.DLGName`)))

(fn `ModifyBoolValue`
  (params (ValueName :type Name) (bNewValue :type Boolean))
  (returns (ReturnValue :type Boolean))
  (return false))

(fn `ModifyFloatValue`
  (params (ValueName :type Name) (bDelta :type Boolean) (Value :type "Float (single-precision)"))
  (returns (ReturnValue :type Boolean))
  (return false))

(fn `ModifyIntValue`
  (params (ValueName :type Name) (bDelta :type Boolean) (Value :type Integer))
  (returns (ReturnValue :type Boolean))
  (return false))

(fn `ModifyNameValue`
  (params (ValueName :type Name) (NameValue :type Name))
  (returns (ReturnValue :type Boolean))
  (return false))

(fn `OnDialogueEvent`
  (params (Context :type "DlgContext Object Reference") (EventName :type Name))
  (returns (ReturnValue :type Boolean))
  (return false))

(fn `UserConstructionScript`)