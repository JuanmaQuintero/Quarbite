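; AI controller for the NPC that follows the player, patrols or walks to a phone location.
; It starts BT_NPC and runs a self-repeating AIMoveTo follow loop toward the player position cached on Tick.
; Patrol picks one of three collected PatrollingSpot1 locations at random, with a longer search pause at the last index.
; GoToPhone halts following for a hardcoded destination, while near/away events only set a waiting flag.
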(event `self.ReceiveBeginPlay`
  (`self.RunBehaviorTree` "/Game/ProjectContent/BluePrints/NPC/BT_NPC.BT_NPC")
  (bind _returnvalue (`GameplayStatics.GetActorOfClass` "/Game/ProjectContent/Character/Animations/Ivan/Telephone/BP_Phone.BP_Phone_C"))
  (set `self.PhonePos` _returnvalue)
  (bind _asbp_main_character (cast `/Game/ProjectContent/BluePrints/Character/BP_MainCharacter` (`GameplayStatics.GetPlayerPawn` 0)))
  (set `self.Character Ref` _asbp_main_character)
  (bind _returnvalue_2 (`GameplayStatics.GetActorOfClass` "/Game/ProjectContent/BluePrints/NPC/BP_NPC.BP_NPC_C"))
  (set `self.NPC` _returnvalue_2)
  (bind _returnvalue_3 (`GameplayStatics.GetActorOfClass` "/Game/ProjectContent/BluePrints/NPC/BP_GarageSpot.BP_GarageSpot_C"))
  (set `self.garageSpot` _returnvalue_3)
  (`self.MoveToPlayer`)
  (bind _outactors (`GameplayStatics.GetAllActorsOfClass` "/Game/ProjectContent/BluePrints/NPC/BP_PatrollingSpot1.BP_PatrollingSpot1_C"))
  (for _array_element _outactors
    (`KismetArrayLibrary.Array_Add` (`self.patrollingPath`) (`self.K2_GetActorLocation` _array_element))))

(event `MoveToPlayer`
  (if (not (`self.stopfollowing`))
    (if (not (`/Game/ProjectContent/BluePrints/NPC/BP_NPC.isPatrolling` (`self.NPC`)))
      (`KismetSystemLibrary.Delay` 0.4)
      (`|AIMoveTo` null (`self.Player POS`) null 150.0
        (:`OnSuccess`
          _)
        (:`OnFail`
          _))
      (`self.MoveToPlayer`))))

(event `self.ReceiveTick`
  (params (DeltaSeconds :type "Float (single-precision)"))
  (if (not (`/Game/ProjectContent/BluePrints/NPC/BP_NPC.isPatrolling` (`self.NPC`)))
    (set `self.Player POS` (`self.K2_GetActorLocation` (`self.Character Ref`)))))

(event `Patrol`
  (if (`/Game/ProjectContent/BluePrints/NPC/BP_NPC.isPatrolling` (`self.NPC`))
    (bind _output_get (set `self.wichOne` (`KismetMathLibrary.RandomIntegerInRange` 0 2)))
    (bind _movementresult (`|AIMoveTo` null (`|GetArrayItem` (`self.patrollingPath`) _output_get) null)
      (:`OnSuccess`
        (`KismetSystemLibrary.PrintString` "he arribat")
        (if (== _output_get 2)
          (set `/Game/ProjectContent/BluePrints/NPC/BP_NPC.doSearch` true (`self.NPC`))
          (`KismetSystemLibrary.Delay` 12.0)
          (set `/Game/ProjectContent/BluePrints/NPC/BP_NPC.doSearch` false (`self.NPC`))
          (`self.Patrol`)
          (else
            (`KismetSystemLibrary.Delay` 4.0)
            (`self.Patrol`))))
      (:`OnFail`
        (`KismetSystemLibrary.PrintString` (`|GetEnumeratorNameAsString` _movementresult))))))

(event `PlayerNear`
  (set `self.isWaiting` true)
  (`KismetSystemLibrary.PrintString` "parate"))

(event `PlayerAway`
  (set `self.isWaiting` false)
  (`KismetSystemLibrary.PrintString` "patrullea otra vez"))

(event `waitInGarage`)

(event `GoToPhone`
  (set `self.stopfollowing` true)
  (`|AIMoveTo` null (1859.748635 -271.617011 86.388843) null 10.0))

(fn `PlayerNearAway`
  (returns (NewParam :type Boolean))
  (return (`self.isWaiting`)))

(fn `UserConstructionScript`)