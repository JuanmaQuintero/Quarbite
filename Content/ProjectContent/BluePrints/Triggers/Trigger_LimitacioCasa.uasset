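; Trigger_LimitacioCasa is a box trigger, sized from exposed variables, that reacts when the main character enters it.
; With JustStop set, it turns the player toward a look target and shows a temporary Catalan "can't go this way yet" message through BP_UIManager.
; Otherwise, it flags the player that the NPC stops following, switches BP_NPC to patrolling through its AI controller, and destroys itself.
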(event `self.ReceiveBeginPlay`
  (bind _returnvalue (`GameplayStatics.GetActorOfClass` "/Game/ProjectContent/BluePrints/Character/BP_UIManager.BP_UIManager_C"))
  (set `self.UIManager` _returnvalue)
  (bind _returnvalue_2 (`GameplayStatics.GetActorOfClass` "/Game/ProjectContent/BluePrints/NPC/BP_NPC.BP_NPC_C"))
  (set `self.NPC` _returnvalue_2))

(event `self.Box.OnComponentBeginOverlap`
  (params (OverlappedComponent :type "PrimitiveComponent Object Reference") (OtherActor :type "Actor Object Reference") (OtherComp :type "PrimitiveComponent Object Reference") (OtherBodyIndex :type Integer) (bFromSweep :type Boolean) (SweepResult :type "HitResult Structure (by ref)"))
  (bind _npc (`self.NPC`))
  (bind _uimanager (`self.UIManager`))
  (bind _asbp_main_character (cast `/Game/ProjectContent/BluePrints/Character/BP_MainCharacter` OtherActor))
  (if (`self.justStop`)
    (message `/Game/ProjectContent/Interfaces/I_LookAt.LookAt` _asbp_main_character (`self.Target to Look`))
    (`TextBlock.SetText` (`/Game/ProjectContent/UI/W_Help.TextToChange` (`/Game/ProjectContent/BluePrints/Character/BP_UIManager.Help` _uimanager)) "Encara no pots anar per aqui.")
    (`/Game/ProjectContent/BluePrints/Character/BP_UIManager.Show HelpUI` _uimanager)
    (`KismetSystemLibrary.Delay` 3.0)
    (`/Game/ProjectContent/BluePrints/Character/BP_UIManager.Hide HelpUI` (`self.UIManager`))
    (else
      (`KismetSystemLibrary.PrintString` "NPC da parte Ouija")
      (`GameplayStatics.GetActorOfClass` "/Game/ProjectContent/BluePrints/NPC/BP_NPC.BP_NPC_C")
      (bind _asbp_main_character_2 (cast `/Game/ProjectContent/BluePrints/Character/BP_MainCharacter` (`GameplayStatics.GetPlayerPawn` 0)))
      (set `/Game/ProjectContent/BluePrints/Character/BP_MainCharacter.NPCStopsFollowing` true _asbp_main_character_2)
      (bind _asaic_npccontroller (cast `/Game/ProjectContent/BluePrints/NPC/AIC_NPCController` (`AIBlueprintHelperLibrary.GetAIController` _npc)))
      (set `/Game/ProjectContent/BluePrints/NPC/BP_NPC.isPatrolling` true _npc)
      (`/Game/ProjectContent/BluePrints/NPC/AIC_NPCController.Patrol` _asaic_npccontroller)
      (`self.K2_DestroyActor`))))

(fn `UserConstructionScript`
  (`BoxComponent.SetBoxExtent` (`self.Box`) (`KismetMathLibrary.MakeVector` (`self.X`) (`self.Y`) (`self.Z`)) true))