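; Storage trigger volume that directs the main character's attention to the level's BP_SafeBox.
; It finds the safe box at BeginPlay and passes it to the character's LookAtMessage when the character overlaps the Box.
; Its DoActions override calls the parent, clears the player character's ShouldSound flag and destroys the trigger; nothing in this graph calls it.
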(event `self.ReceiveBeginPlay`
  (`parent.ReceiveBeginPlay`)
  (bind _returnvalue (`GameplayStatics.GetActorOfClass` "/Game/ProjectContent/BluePrints/Puzles/BP_SafeBox.BP_SafeBox_C"))
  (set `self.SafeBox` _returnvalue))

(event `self.Box.OnComponentBeginOverlap`
  (params (OverlappedComponent :type "PrimitiveComponent Object Reference") (OtherActor :type "Actor Object Reference") (OtherComp :type "PrimitiveComponent Object Reference") (OtherBodyIndex :type Integer) (bFromSweep :type Boolean) (SweepResult :type "HitResult Structure (by ref)"))
  (bind _asbp_main_character (cast `/Game/ProjectContent/BluePrints/Character/BP_MainCharacter` OtherActor))
  (message `/Game/ProjectContent/Interfaces/I_LookAt.LookAt` _asbp_main_character (`self.SafeBox`)))

(fn `DoActions`
  (`parent.DoActions`)
  (bind _asbp_main_character (cast `/Game/ProjectContent/BluePrints/Character/BP_MainCharacter` (`GameplayStatics.GetPlayerPawn` 0)))
  (set `/Game/ProjectContent/BluePrints/Character/BP_MainCharacter.ShouldSound` false _asbp_main_character)
  (`self.K2_DestroyActor`))

(fn `UserConstructionScript`
  (`parent.UserConstructionScript`))