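; Bathroom trigger, a child of a parent trigger class, that turns off the shower sound.
; On BeginPlay it caches the Trigger_SombraEsquina actor as the sound origin.
; Its DoActions override runs the parent logic, stops that actor's sound and spawns a shower-closing cue at a hardcoded world location.
; It then prints a debug message and destroys itself, making it one-shot.
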(event `self.ReceiveBeginPlay`
  (`parent.ReceiveBeginPlay`)
  (bind _returnvalue (`GameplayStatics.GetActorOfClass` "/Game/ProjectContent/BluePrints/Triggers/Trigger_SombraEsquina.Trigger_SombraEsquina_C"))
  (set `self.SoundOrigin` _returnvalue))

(fn `DoActions`
  (`parent.DoActions`)
  (`AudioComponent.Stop` (`/Game/ProjectContent/BluePrints/Triggers/Trigger_SombraEsquina.Sound` (`self.SoundOrigin`)))
  (bind _returnvalue (`GameplayStatics.SpawnSoundAtLocation` "/Game/ProjectContent/Music/Shower/ShowerClose_Cue1.ShowerClose_Cue1" (1614.918031 -1616.378375 190.315906) (struct) 1.0 1.0 0.0 null null))
  (set `self.Sound` _returnvalue)
  (`KismetSystemLibrary.PrintString` "Parar sonido ducha")
  (`self.K2_DestroyActor`))

(fn `UserConstructionScript`
  (`parent.UserConstructionScript`))