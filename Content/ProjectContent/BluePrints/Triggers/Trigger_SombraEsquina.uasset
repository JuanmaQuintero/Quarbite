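; Scripted horror trigger that stages a shadow apparition and its disappearance.
; The overridden DoActions spawns BP_Shadow at a fixed spot, triggers temporary full panic, turns the player toward BP_SombraSpot2 and plays a sound.
; Player overlap with the box starts a delayed vanish that briefly cuts the flashlight, destroys the shadow, starts a shower sound and disables the box collision.
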(event `self.ReceiveBeginPlay`
  (`parent.ReceiveBeginPlay`)
  (bind _returnvalue (`GameplayStatics.GetActorOfClass` "/Game/ProjectContent/BluePrints/BP_SombraSpot2.BP_SombraSpot2_C"))
  (set `self.LookAtPos` _returnvalue)
  (bind _returnvalue_2 (`GameplayStatics.GetActorOfClass` "/Game/ProjectContent/BluePrints/Items/BP_FlashLight.BP_FlashLight_C"))
  (set `self.FlashLight` _returnvalue_2)
  (bind _returnvalue_3 (`GameplayStatics.GetActorOfClass` "/Game/ProjectContent/BluePrints/Managers/BP_PanicManager.BP_PanicManager_C"))
  (set `self.PanicManager` _returnvalue_3))

(event `self.Box.OnComponentBeginOverlap`
  (params (OverlappedComponent :type "PrimitiveComponent Object Reference") (OtherActor :type "Actor Object Reference") (OtherComp :type "PrimitiveComponent Object Reference") (OtherBodyIndex :type Integer) (bFromSweep :type Boolean) (SweepResult :type "HitResult Structure (by ref)"))
  (bind _asbp_main_character (cast `/Game/ProjectContent/BluePrints/Character/BP_MainCharacter` OtherActor))
  (set `self.Main Character` _asbp_main_character)
  (`KismetSystemLibrary.Delay` 4.0)
  (`self.Desaparece`))

(event `Desaparece`
  (`/Game/ProjectContent/BluePrints/Items/BP_FlashLight.TurnOff` (`self.FlashLight`))
  (`self.K2_DestroyActor` (`self.Ombra`))
  (`KismetSystemLibrary.Delay` 0.5)
  (`/Game/ProjectContent/BluePrints/Items/BP_FlashLight.TurnOn` (`self.FlashLight`))
  (bind _returnvalue (`GameplayStatics.SpawnSoundAtLocation` "/Game/ProjectContent/Music/Shower/ShowerNormal_Cue.ShowerNormal_Cue" (1614.918031 -1616.378375 190.315906) (struct) 1.0 1.0 0.0 null null))
  (set `self.Sound` _returnvalue)
  (`PrimitiveComponent.SetCollisionEnabled` (`self.Box`) "NoCollision"))

(fn `DoActions`
  (`parent.DoActions`)
  (bind _returnvalue (`AIBlueprintHelperLibrary.SpawnAIFromClass` "/Game/ProjectContent/BluePrints/Shadow/BP_Shadow.BP_Shadow_C" null (1946.378888 -1338.377705 91.000063) (struct :`Yaw` 10.0) false null))
  (set `self.Ombra` _returnvalue)
  (`/Game/ProjectContent/BluePrints/Managers/BP_PanicManager.FullPanicTemporary` (`self.PanicManager`))
  (bind _asbp_main_character (cast `/Game/ProjectContent/BluePrints/Character/BP_MainCharacter` (`GameplayStatics.GetPlayerPawn` 0)))
  (`/Game/ProjectContent/Interfaces/I_LookAt.LookAt` _asbp_main_character (`self.LookAtPos`))
  (`GameplayStatics.PlaySound2D` "/Game/ProjectContent/Music/Panic/Segundo.Segundo" 1.0 1.0 0.0 null null))

(fn `UserConstructionScript`
  (`parent.UserConstructionScript`))