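; Trigger volume that directs the main character's attention to a target and, when its actions run, makes picture frame actors grabbable.
; BeginPlay caches one actor each of three frame classes, and box overlap by BP_MainCharacter sends LookAtMessage with TargetToLook.
; The DoActions override enables CanGrab, then destroys the trigger.
; DoActions sets Frame2 twice and never Frame1, so only Frame2 and Frame3 become grabbable.
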(event `self.ReceiveBeginPlay`
  (`parent.ReceiveBeginPlay`)
  (bind _returnvalue (`GameplayStatics.GetActorOfClass` "/Game/ProjectContent/BluePrints/Puzles/BP_Frame1.BP_Frame1_C"))
  (set `self.Frame 1` _returnvalue)
  (bind _returnvalue_2 (`GameplayStatics.GetActorOfClass` "/Game/ProjectContent/BluePrints/Puzles/BP_Frame.BP_Frame_C"))
  (set `self.Frame 2` _returnvalue_2)
  (bind _returnvalue_3 (`GameplayStatics.GetActorOfClass` "/Game/ProjectContent/BluePrints/Puzles/BP_Frame2.BP_Frame2_C"))
  (set `self.Frame 3` _returnvalue_3))

(event `self.Box.OnComponentBeginOverlap`
  (params (OverlappedComponent :type "PrimitiveComponent Object Reference") (OtherActor :type "Actor Object Reference") (OtherComp :type "PrimitiveComponent Object Reference") (OtherBodyIndex :type Integer) (bFromSweep :type Boolean) (SweepResult :type "HitResult Structure (by ref)"))
  (bind _asbp_main_character (cast `/Game/ProjectContent/BluePrints/Character/BP_MainCharacter` OtherActor))
  (message `/Game/ProjectContent/Interfaces/I_LookAt.LookAt` _asbp_main_character (`self.Target to Look`)))

(fn `DoActions`
  (`parent.DoActions`)
  (set `/Game/ProjectContent/BluePrints/Puzles/BP_Frame.canGrab?` true (`self.Frame 2`))
  (set `/Game/ProjectContent/BluePrints/Puzles/BP_Frame.canGrab?` true (`self.Frame 2`))
  (set `/Game/ProjectContent/BluePrints/Puzles/BP_Frame2.canGrab?` true (`self.Frame 3`))
  (`self.K2_DestroyActor`))

(fn `UserConstructionScript`
  (`parent.UserConstructionScript`))