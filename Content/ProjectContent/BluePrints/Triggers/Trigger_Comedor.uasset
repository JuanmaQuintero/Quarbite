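; Dining-room (Comedor) trigger that moves a movable chair as a one-shot scripted action.
; On BeginPlay it caches a BP_ChairMovable found in the level through GetActorOfClass.
; Its DoActions override runs the parent logic, calls Move on that chair, then destroys the trigger; activation is left to the parent class, as its own overlap event is disabled.
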(event `self.ReceiveBeginPlay`
  (`parent.ReceiveBeginPlay`)
  (bind _returnvalue (`GameplayStatics.GetActorOfClass` "/Game/ProjectContent/BluePrints/PropsInteractuables/BP_ChairMovable.BP_ChairMovable_C"))
  (set `self.Chair` _returnvalue))

(fn `DoActions`
  (`parent.DoActions`)
  (`/Game/ProjectContent/BluePrints/PropsInteractuables/BP_ChairMovable.Move` (`self.Chair`))
  (`self.K2_DestroyActor`))

(fn `UserConstructionScript`
  (`parent.UserConstructionScript`))