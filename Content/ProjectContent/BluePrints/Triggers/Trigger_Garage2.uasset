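; Garage trigger that, when its actions fire, lifts the house boundary restriction and then destroys itself.
; On BeginPlay it caches the Trigger_LimitacioCasa actor, and its DoActions override clears that actor's JustStop flag.
; Limiting fuse interaction and the NPC audio hint to explore exist only as debug print placeholders.
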(event `self.ReceiveBeginPlay`
  (`parent.ReceiveBeginPlay`)
  (bind _returnvalue (`GameplayStatics.GetActorOfClass` "/Game/ProjectContent/BluePrints/Triggers/Trigger_LimitacioCasa.Trigger_LimitacioCasa_C"))
  (set `self.Limitator` _returnvalue))

(fn `DoActions`
  (`parent.DoActions`)
  (`KismetSystemLibrary.PrintString` "Limitar la interaccion de los fusibles")
  (`KismetSystemLibrary.PrintString` "Desbloquear limitación casa")
  (`KismetSystemLibrary.PrintString` "Audio NPC indicando de explorar")
  (set `/Game/ProjectContent/BluePrints/Triggers/Trigger_LimitacioCasa.justStop` false (`self.Limitator`))
  (`self.K2_DestroyActor`))

(fn `UserConstructionScript`
  (`parent.UserConstructionScript`))