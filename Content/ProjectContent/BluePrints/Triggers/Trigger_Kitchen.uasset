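; Kitchen trigger Blueprint that stages a power-outage event by switching off the lights and flagging the fuse box.
; Its DoActions override calls the parent, advances BP_NPC dialogue, runs ApagarLuces, marks BP_Fusibles unsolved with the light out, then destroys itself.
; ApagarLuces turns off every BP_Switch and, redundantly inside that loop, the single BP_Switch1.
; Flicker stop and UI message are only debug prints.
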(event `ApagarLuces`
  (bind _outactors (`GameplayStatics.GetAllActorsOfClass` "/Game/ProjectContent/BluePrints/PropsInteractuables/BP_Switch.BP_Switch_C"))
  (for _array_element _outactors
    (set `/Game/ProjectContent/BluePrints/PropsInteractuables/BP_Switch.isOn` false _array_element)
    (`/Game/ProjectContent/BluePrints/PropsInteractuables/BP_Switch.CheckState` _array_element)
    (bind _returnvalue (`GameplayStatics.GetActorOfClass` "/Game/ProjectContent/BluePrints/PropsInteractuables/BP_Switch1.BP_Switch1_C"))
    (set `/Game/ProjectContent/BluePrints/PropsInteractuables/BP_Switch1.isOn` false _returnvalue)
    (`/Game/ProjectContent/BluePrints/PropsInteractuables/BP_Switch1.CheckState` _returnvalue)))

(fn `DoActions`
  (`parent.DoActions`)
  (`KismetSystemLibrary.PrintString` "Luz deja de parpadear")
  (`KismetSystemLibrary.PrintString` "Apagar luces")
  (`KismetSystemLibrary.PrintString` "Mensajito UI \"Parece que le ha pasado algo al cuadro de luces\"")
  (bind _returnvalue (`GameplayStatics.GetActorOfClass` "/Game/ProjectContent/BluePrints/NPC/BP_NPC.BP_NPC_C"))
  (set `/Game/ProjectContent/BluePrints/NPC/BP_NPC.dialogStart` 11 _returnvalue)
  (`self.ApagarLuces`)
  (bind _returnvalue_2 (`GameplayStatics.GetActorOfClass` "/Game/ProjectContent/BluePrints/Puzles/BP_Fusibles.BP_Fusibles_C"))
  (set `/Game/ProjectContent/BluePrints/Puzles/BP_Fusibles.solved` false _returnvalue_2)
  (set `/Game/ProjectContent/BluePrints/Puzles/BP_Fusibles.lightWentOff` true _returnvalue_2)
  (`self.K2_DestroyActor`))

(fn `UserConstructionScript`
  (`parent.UserConstructionScript`))