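; BP_ProbaBuzon is an interactable mailbox prop whose mouth (BocaBuzon) swings open and closed.
; Interaction works only while the cached main character can begin to search and the Abrir timeline is idle.
; It toggles IsOpened and plays or reverses that timeline to yaw the mouth up to 90 degrees.
; Highlight events set or clear an overlay material on the mouth, while the Interact function is an empty stub.
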(event `self.ReceiveBeginPlay`
  ; Begin Play
  (bind _asbp_main_character (cast `/Game/ProjectContent/BluePrints/Character/BP_MainCharacter` (`GameplayStatics.GetPlayerCharacter` 0)))
  (set `self.Character Ref` _asbp_main_character)
  (set `self.IsOpened` false))

(event `/Game/ProjectContent/Interfaces/I_Interact.Interaction`
  (params (Interactor :type "Character Object Reference") (ItemToPut :type "/Game/ProjectContent/BluePrints/Items/BP_InteractionItem Object Reference") (ComponentHit :type "ActorComponent Object Reference"))
  ; Interaction
  (if (`/Game/ProjectContent/BluePrints/Character/BP_MainCharacter.canBeginToSearch` (`self.Character Ref`))
    (if (not (`TimelineComponent.IsPlaying` (`self.Abrir`)))
      (if (not (`self.IsOpened`))
        (set `self.IsOpened` true)
        (bind (_direction _newtrack_0) (`Timeline|Abrir` :!via `PlayFromStart` :!label _label)
          (:`Update`
            (`SceneComponent.K2_SetRelativeRotation` (`self.BocaBuzon`) (`KismetMathLibrary.MakeRotator` 0.0 0.0 (* _newtrack_0 90.0)) false false)))
        (else
          (set `self.IsOpened` false)
          (goto _label :!via `ReverseFromEnd`))))))

(event `/Game/ProjectContent/Interfaces/I_Interact.HighLightItem`
  (`MeshComponent.SetOverlayMaterial` (`self.BocaBuzon`) "/Game/ProjectContent/Material/Ligths/M_HighLight2_Inst.M_HighLight2_Inst"))

(event `/Game/ProjectContent/Interfaces/I_Interact.StopHighLightItem`
  (`MeshComponent.SetOverlayMaterial` (`self.BocaBuzon`) null))

(fn `Interact`
  (params (Interactor :type "Character Object Reference"))
  (return))

(fn `UserConstructionScript`)