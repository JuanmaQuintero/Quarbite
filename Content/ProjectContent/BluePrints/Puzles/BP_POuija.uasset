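; BP_POuija is a pickup puzzle piece for the Ouija table puzzle.
; On BeginPlay it finds and caches the BP_OuijaTable actor in the level.
; Its DoPick override runs the parent pick logic, adds its ItemData to the table, flags the player's BP_MainCharacter as having a piece, then destroys itself.
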(event `self.ReceiveBeginPlay`
  (bind _returnvalue (`GameplayStatics.GetActorOfClass` "/Game/ProjectContent/BluePrints/Puzles/BP_OuijaTable.BP_OuijaTable_C"))
  (set `self.Ouija Table` _returnvalue))

(fn `DoPick`
  (`parent.DoPick`)
  (`/Game/ProjectContent/BluePrints/Puzles/BP_OuijaTable.AddPieceToTable` (`self.Ouija Table`) (`self.ItemData`))
  (bind _asbp_main_character (cast `/Game/ProjectContent/BluePrints/Character/BP_MainCharacter` (`GameplayStatics.GetPlayerPawn` 0)))
  (set `/Game/ProjectContent/BluePrints/Character/BP_MainCharacter.hasPiece` true _asbp_main_character)
  (`self.K2_DestroyActor`))

(fn `UserConstructionScript`
  (`parent.UserConstructionScript`))