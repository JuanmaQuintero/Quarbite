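; Combination lock puzzle that the player inspects up close, switching to the lock's view and puzzle mode with the HUD hidden until exit.
; BeginPlay spawns three dials on Body sockets, each given an index and lock reference.
; CheckEveryTurn compares dial numbers with LockCombination.
; A match runs chained timelines that lift and rotate the latch, mark the lock unlocked, then drop body and latch after a short delay.
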(event `self.ReceiveBeginPlay`
  (bind _asbp_main_character (cast `/Game/ProjectContent/BluePrints/Character/BP_MainCharacter` (`GameplayStatics.GetPlayerPawn` 0)))
  (set `self.As BP Main Character` _asbp_main_character)
  (for _index (range 3)
    (bind _returnvalue (`|SpawnActorFromClass` "/Game/ProjectContent/BluePrints/Puzles/BP_Dial.BP_Dial_C" (`KismetMathLibrary.MakeTransform` (0.0 0.0 0.0) (struct :`Yaw` 144.0)) "Undefined" "MultiplyWithRoot" null _index self null))
    (`KismetArrayLibrary.Array_Add` (`self.Dials`) _returnvalue)
    (`self.K2_AttachToComponent` _returnvalue (`self.Body`) (select `int` _index :`0` "Dial01" :`1` "Dial02" :`2` "Dial03" :!type "Name") "KeepRelative" "KeepRelative" "KeepRelative" true)
    (`self.EnableInput` (`GameplayStatics.GetPlayerController` 0))
    (set `self.X` (.x (`SceneComponent.RelativeLocation` (`self.Latch1`))))
    (set `self.Y` (.y (`SceneComponent.RelativeLocation` (`self.Latch1`))))
    (set `self.Z` (.z (`SceneComponent.RelativeLocation` (`self.Latch1`))))))

(event `/Game/ProjectContent/Interfaces/I_Interact.Interaction`
  (params (Interactor :type "Character Object Reference") (ItemToPut :type "/Game/ProjectContent/BluePrints/Items/BP_InteractionItem Object Reference") (ComponentHit :type "ActorComponent Object Reference"))
  (bind _as_bp_main_character (`self.As BP Main Character`))
  (if (not (`self.unlucked`))
    (set `self.IsInLock` true)
    (`PlayerController.SetViewTargetWithBlend` (`GameplayStatics.GetPlayerController` 0) self 0.5 "VTBlend_Linear" 0.0 false)
    (`/Game/ProjectContent/BluePrints/Character/BP_MainCharacter.goPuzleMode` _as_bp_main_character)
    (`/Game/ProjectContent/BluePrints/Character/BP_MainCharacter.HideHUD` _as_bp_main_character)))

(event `EnhancedInput|/Game/ProjectContent/Inputs/InputsPuzle/IA_GoOutOfPuzzle`
  (params (ActionValue :type Boolean) (ElapsedSeconds :type "Float (double-precision)") (TriggeredSeconds :type "Float (double-precision)") (InputAction :type "InputAction Object Reference" :default "/Game/ProjectContent/Inputs/InputsPuzle/IA_GoOutOfPuzzle.IA_GoOutOfPuzzle"))
  (:`Started`
    (if (`self.IsInLock`)
      (`PlayerController.SetViewTargetWithBlend` (`GameplayStatics.GetPlayerController` 0) (`GameplayStatics.GetPlayerPawn` 0) 0.5 "VTBlend_Linear" 0.0 false)
      (set `self.IsInLock` false)
      (`/Game/ProjectContent/BluePrints/Character/BP_MainCharacter.goNormalMode` (`self.As BP Main Character`))
      (`/Game/ProjectContent/BluePrints/Character/BP_MainCharacter.ShowHUD` (`self.As BP Main Character`)))))

(event `CheckEveryTurn`
  (bind _success (`self.CheckCode`))
  (if _success
    (`self.UnlockLock`)))

(event `UnlockLock`
  (bind (_direction _newtrack_0) (`Timeline|Timeline` :!via `PlayFromStart`)
    (:`Update`
      (`SceneComponent.K2_SetRelativeLocation` (`self.Latch1`) (`KismetMathLibrary.MakeVector` (`self.X`) (`self.Y`) (+ (* _newtrack_0 2.0) (`self.Z`))) false false))
    (:`Finished`
      (bind (_direction_2 _newtrack_0_2) (`Timeline|Timeline_0` :!via `PlayFromStart`)
        (:`Update`
          (`SceneComponent.K2_SetRelativeRotation` (`self.Latch1`) (`KismetMathLibrary.MakeRotator` 0.0 0.0 (* _newtrack_0_2 90.0)) false false))
        (:`Finished`
          (set `self.unlucked` true)
          (`KismetSystemLibrary.Delay` 0.3)
          (bind (_direction_3 _newtrack_0_3) (`Timeline|Timeline_1`)
            (:`Update`
              (`SceneComponent.K2_SetRelativeLocation` (`self.Body`) (`KismetMathLibrary.MakeVector` (`self.X`) (`self.Y`) (* _newtrack_0_3 -25.0)) false false)
              (`SceneComponent.K2_SetRelativeLocation` (`self.Latch1`) (`KismetMathLibrary.MakeVector` (`self.X`) (`self.Y`) (* _newtrack_0_3 -25.0)) false false))))))))

(fn `CheckCode`
  (returns (Success :type Boolean))
  (locals (LocalSuccess :type Boolean))
  (for (_array_element _array_index) (`self.Dials`)
    (if (== (`/Game/ProjectContent/BluePrints/Puzles/BP_Dial.Number` _array_element) (`|GetArrayItem` (`self.LockCombination`) _array_index))
      (`KismetSystemLibrary.PrintString` "Hello")
      (set `local.LocalSuccess` true)
      (else
        (set `local.LocalSuccess` false)
        (break))))
  (return (`local.LocalSuccess`)))

(fn `UserConstructionScript`)