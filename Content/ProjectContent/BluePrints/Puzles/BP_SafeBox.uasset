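; Keypad safe puzzle that the player opens with a hardcoded code to collect a Ouija piece.
; Interaction blends the camera to the safe and puts the character in puzzle mode.
; Clicked keys animate and append digits; Enter counts positional matches against the solution.
; Success plays chained wheel and door timelines, raises a global emissive parameter and shows the help prompt, enabling pickup through Enhanced Input.
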(event `self.ReceiveBeginPlay`
  (set `self.solution` (`|MakeArray` 2 2 6 6 2))
  (bind _asbp_main_character (cast `/Game/ProjectContent/BluePrints/Character/BP_MainCharacter` (`GameplayStatics.GetPlayerPawn` 0)))
  (set `self.As BP Main Character` _asbp_main_character)
  (`self.EnableInput` (`GameplayStatics.GetPlayerController` 0))
  (bind _returnvalue (`GameplayStatics.GetActorOfClass` "/Game/ProjectContent/BluePrints/Character/BP_UIManager.BP_UIManager_C"))
  (set `self.UIManager` _returnvalue))

(event `Animacion de abrir`
  (bind (_direction _newtrack_0) (`Timeline|MoveWheel`)
    (:`Update`
      (`SceneComponent.K2_SetRelativeRotation` (`self.wheel`) (`KismetMathLibrary.MakeRotator` (* _newtrack_0 180.0)) false false))
    (:`Finished`
      (bind (_direction_2 _newtrack_0_2) (`Timeline|Open Door`)
        (:`Update`
          (`SceneComponent.K2_SetRelativeRotation` (`self.tape`) (`KismetMathLibrary.MakeRotator` 0.0 0.0 (* _newtrack_0_2 -75.0)) false false))
        (:`Finished`
          (set `self.puertaAbierta` true)
          (`/Game/ProjectContent/BluePrints/Character/BP_UIManager.Show HelpUI` (`self.UIManager`))
          (`TextBlock.SetText` (`/Game/ProjectContent/UI/W_Help.TextToChange` (`/Game/ProjectContent/BluePrints/Character/BP_UIManager.Help` (`self.UIManager`))) "Presiona la tecla \"E\" para coger la pieza de Ouija"))))))

(event `/Game/ProjectContent/Interfaces/I_Interact.Interaction`
  (params (Interactor :type "Character Object Reference") (ItemToPut :type "/Game/ProjectContent/BluePrints/BP_InteractionItem Object Reference") (ComponentHit :type "ActorComponent Object Reference"))
  (`self.StopHighLightItem`)
  (`PlayerController.SetViewTargetWithBlend` (`GameplayStatics.GetPlayerController` 0) self 1.0 "VTBlend_Linear" 0.0 false)
  (`/Game/ProjectContent/BluePrints/Character/BP_MainCharacter.goPuzleMode` (`self.As BP Main Character`))
  (set `self.isInSafeBox` true))

(event `EnhancedInput|/Game/ProjectContent/Inputs/InputsPuzle/IA_PickItemInside`
  (params (ActionValue :type Boolean) (ElapsedSeconds :type "Float (double-precision)") (TriggeredSeconds :type "Float (double-precision)") (InputAction :type "InputAction Object Reference" :default "/Game/ProjectContent/Inputs/InputsPuzle/IA_PickItemInside.IA_PickItemInside"))
  (:`Started`
    (if (`self.puertaAbierta`)
      (`KismetSystemLibrary.PrintString` "Coger pieza")
      (`/Game/ProjectContent/BluePrints/BP_InteractionItem.DoPick` (`self.OuijaPiece`))
      (`/Game/ProjectContent/BluePrints/Character/BP_UIManager.Hide HelpUI` (`self.UIManager`)))))

(event `self.1.OnClicked`
  (params (TouchedComponent :type "PrimitiveComponent Object Reference") (ButtonPressed :type "Key Structure"))
  (`self.addNumber` 1 TouchedComponent))

(event `self.2.OnClicked`
  (params (TouchedComponent :type "PrimitiveComponent Object Reference") (ButtonPressed :type "Key Structure"))
  (`self.addNumber` 2 TouchedComponent))

(event `self.3.OnClicked`
  (params (TouchedComponent :type "PrimitiveComponent Object Reference") (ButtonPressed :type "Key Structure"))
  (`self.addNumber` 3 TouchedComponent))

(event `EnhancedInput|/Game/ProjectContent/Inputs/InputsPuzle/IA_GoOutOfPuzzle`
  (params (ActionValue :type Boolean) (ElapsedSeconds :type "Float (double-precision)") (TriggeredSeconds :type "Float (double-precision)") (InputAction :type "InputAction Object Reference" :default "/Game/ProjectContent/Inputs/InputsPuzle/IA_GoOutOfPuzzle.IA_GoOutOfPuzzle"))
  (:`Triggered`
    (if (`self.isInSafeBox`)
      (`PlayerController.SetViewTargetWithBlend` (`GameplayStatics.GetPlayerController` 0) (`GameplayStatics.GetPlayerPawn` 0) 0.5 "VTBlend_Linear" 0.0 false)
      (`/Game/ProjectContent/BluePrints/Character/BP_MainCharacter.goNormalMode` (`self.As BP Main Character`))
      (set `self.isInSafeBox` false)
      (`/Game/ProjectContent/BluePrints/Character/BP_UIManager.Hide HelpUI` (`self.UIManager`)))))

(event `self.4.OnClicked`
  (params (TouchedComponent :type "PrimitiveComponent Object Reference") (ButtonPressed :type "Key Structure"))
  (`self.addNumber` 4 TouchedComponent))

(event `self.5.OnClicked`
  (params (TouchedComponent :type "PrimitiveComponent Object Reference") (ButtonPressed :type "Key Structure"))
  (`self.addNumber` 5 TouchedComponent))

(event `self.6.OnClicked`
  (params (TouchedComponent :type "PrimitiveComponent Object Reference") (ButtonPressed :type "Key Structure"))
  (`self.addNumber` 6 TouchedComponent))

(event `self.7.OnClicked`
  (params (TouchedComponent :type "PrimitiveComponent Object Reference") (ButtonPressed :type "Key Structure"))
  (`self.addNumber` 7 TouchedComponent))

(event `self.8.OnClicked`
  (params (TouchedComponent :type "PrimitiveComponent Object Reference") (ButtonPressed :type "Key Structure"))
  (`self.addNumber` 8 TouchedComponent))

(event `self.9.OnClicked`
  (params (TouchedComponent :type "PrimitiveComponent Object Reference") (ButtonPressed :type "Key Structure"))
  (`self.addNumber` 9 TouchedComponent))

(event `self.erease.OnClicked`
  (params (TouchedComponent :type "PrimitiveComponent Object Reference") (ButtonPressed :type "Key Structure"))
  (`KismetArrayLibrary.Array_Clear` (`self.combination`)))

(event `self.0.OnClicked`
  (params (TouchedComponent :type "PrimitiveComponent Object Reference") (ButtonPressed :type "Key Structure"))
  (`self.addNumber` 0 TouchedComponent))

(event `self.enter.OnClicked`
  (params (TouchedComponent :type "PrimitiveComponent Object Reference") (ButtonPressed :type "Key Structure"))
  (`self.ValidateConbination`))

(event `/Game/ProjectContent/Interfaces/I_Interact.HighLightItem`
  (`MeshComponent.SetOverlayMaterial` (`self.tape`) "/Game/ProjectContent/Material/Ligths/M_HighLight2_Inst.M_HighLight2_Inst"))

(event `/Game/ProjectContent/Interfaces/I_Interact.StopHighLightItem`
  (`MeshComponent.SetOverlayMaterial` (`self.tape`) null))

(event `ButonAnimacion`
  (params (Target :type "SceneComponent Object Reference"))
  (if (not (`TimelineComponent.IsPlaying` (`self.Click`)))
    (bind (_direction _newtrack_0) (`Timeline|Click` :!via `PlayFromStart`)
      (:`Update`
        (`SceneComponent.K2_SetRelativeLocation` Target (`KismetMathLibrary.MakeVector` (* _newtrack_0 -0.25) (.y (`SceneComponent.RelativeLocation` Target)) (.z (`SceneComponent.RelativeLocation` Target))) false false)))))

(fn `addNumber`
  (params (Number :type Integer) (Tecla :type "SceneComponent Object Reference"))
  (`KismetArrayLibrary.Array_Add` (`self.combination`) Number)
  (`KismetSystemLibrary.PrintString` (`KismetStringLibrary.Conv_IntToString` Number))
  (`self.ButonAnimacion` Tecla))

(fn `UserConstructionScript`)

(fn `ValidateConbination`
  (for (_array_element _array_index) (`self.combination`)
    (if (== _array_element (`|GetArrayItem` (`self.solution`) _array_index))
      (`/Engine/EditorBlueprintResources/StandardMacros.IncrementInt` (`self.aciertos`))))
  (if (== (- (`self.aciertos`) 1) (`KismetArrayLibrary.Array_LastIndex` (`self.solution`)))
    (`KismetSystemLibrary.PrintString` "completado")
    (`self.Animacion de abrir`)
    (`KismetArrayLibrary.Array_Clear` (`self.combination`))
    (set `self.aciertos` 0)
    (`KismetMaterialLibrary.SetScalarParameterValue` "/Game/ProjectContent/BluePrints/MPC_Emissive.MPC_Emissive" "Emissive Intensity" 20.0)
    (else
      (`KismetSystemLibrary.PrintString` "no es la clave")
      (`KismetArrayLibrary.Array_Clear` (`self.combination`))
      (set `self.aciertos` 0))))