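; BP_Frame2 is an interactable frame for a puzzle that can be picked up only while CanGrab is true.
; On Interaction it either calls DoPick, which defers to the parent implementation, or briefly shows a Spanish "not possible right now" help message through the BP_UIManager found at BeginPlay.
; A node clearing IsFirstTimeTrying is left unconnected and never runs.
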(event `self.ReceiveBeginPlay`
  (bind _returnvalue (`GameplayStatics.GetActorOfClass` "/Game/ProjectContent/BluePrints/Character/BP_UIManager.BP_UIManager_C"))
  (set `self.UIManager` _returnvalue))

(event `self.Interaction`
  (params (Interactor :type "Character Object Reference") (ItemToPut :type "/Game/ProjectContent/BluePrints/Items/BP_InteractionItem Object Reference") (ComponentHit :type "ActorComponent Object Reference"))
  (bind _uimanager (`self.UIManager`))
  (if (not (`self.canGrab?`))
    (`/Game/ProjectContent/BluePrints/Character/BP_UIManager.Show HelpUI` _uimanager)
    (set `TextBlock.Text` "No es posible en este momento" (`/Game/ProjectContent/UI/W_Help.TextToChange` (`/Game/ProjectContent/BluePrints/Character/BP_UIManager.Help` _uimanager)))
    (`KismetSystemLibrary.Delay` 2.0)
    (`/Game/ProjectContent/BluePrints/Character/BP_UIManager.Hide HelpUI` _uimanager)
    (else
      (`self.DoPick`))))

(fn `DoPick`
  (`parent.DoPick`))

(fn `UserConstructionScript`
  (`parent.UserConstructionScript`))