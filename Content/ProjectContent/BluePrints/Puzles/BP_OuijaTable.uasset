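; Ouija table puzzle actor where the player drags a pointer over letters to spell "CARLES".
; Interaction blends the view to the table and enters puzzle mode; Tick moves the pointer by mouse delta.
; Once all five pieces and the pointer are placed, letters overlapped for one second join the combination via a cancellable timer.
; Release checks the word, only printing the result, clears it and eases the pointer home with a timeline.
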(event `self.ReceiveBeginPlay`
  ; Begin Play
  (bind _asbp_main_character (cast `/Game/ProjectContent/BluePrints/Character/BP_MainCharacter` (`GameplayStatics.GetPlayerPawn` 0)))
  (set `self.CarlesRef` _asbp_main_character)
  (set `self.OriginalLocationPunter` (`SceneComponent.RelativeLocation` (`self.Pointer`)))
  (set `self.solution` (`|MakeArray` "C" "A" "R" "L" "E" "S"))
  (set `self.Meshes` (`|MakeArray` (`self.Pieza1`) (`self.Pieza2`) (`self.Pieza3`) (`self.Pieza4`) (`self.Pieza5`) null))
  (`self.EnableInput` (`GameplayStatics.GetPlayerController` 0)))

(event `/Game/ProjectContent/Interfaces/I_Interact.Interaction`
  (params (Interactor :type "Character Object Reference") (ItemToPut :type "/Game/ProjectContent/BluePrints/BP_InteractionItem Object Reference") (ComponentHit :type "ActorComponent Object Reference"))
  ; Interaction
  (`self.StopHighLightItem`)
  (`PlayerController.SetViewTargetWithBlend` (`GameplayStatics.GetPlayerController` 0) self 1.0 "VTBlend_Linear" 0.0 false)
  (`/Game/ProjectContent/BluePrints/Character/BP_MainCharacter.goPuzleMode` (`self.CarlesRef`))
  (set `self.isInPuzle` true))

(event `EnhancedInput|/Game/ProjectContent/Inputs/InputsPuzle/IA_GoOutOfPuzzle`
  (params (ActionValue :type Boolean) (ElapsedSeconds :type "Float (double-precision)") (TriggeredSeconds :type "Float (double-precision)") (InputAction :type "InputAction Object Reference" :default "/Game/ProjectContent/Inputs/InputsPuzle/IA_GoOutOfPuzzle.IA_GoOutOfPuzzle"))
  (:`Started`
    (if (`self.isInPuzle`)
      (`PlayerController.SetViewTargetWithBlend` (`GameplayStatics.GetPlayerController` 0) (`GameplayStatics.GetPlayerPawn` 0) 0.5 "VTBlend_Linear" 0.0 false)
      (`/Game/ProjectContent/BluePrints/Character/BP_MainCharacter.goNormalMode` (`self.CarlesRef`)))))

(event `self.Pointer.OnClicked`
  (params (TouchedComponent :type "PrimitiveComponent Object Reference") (ButtonPressed :type "Key Structure"))
  (bind (_locationx _locationy) (`PlayerController.GetMousePosition` (`GameplayStatics.GetPlayerController` 0)))
  ; OnClick
  (if (and (not (`TimelineComponent.IsPlaying` (`self.Timeline`))) (`self.isInPuzle`))
    (set `self.isDraging` true)
    (set `self.coneClicked` true)
    (`KismetSystemLibrary.PrintString` "Hello")
    (set `self.ClickedPostion` (`KismetMathLibrary.MakeVector2D` _locationx _locationy))))

(event `self.ReceiveTick`
  (params (DeltaSeconds :type "Float (single-precision)"))
  (bind (_locationx _locationy) (`PlayerController.GetMousePosition` (`GameplayStatics.GetPlayerController` 0)))
  ; OnClick
  (if (`self.isDraging`)
    (if (`self.coneClicked`)
      (bind (_y _x) (`self.CopyMousePosition`))
      (`SceneComponent.K2_AddRelativeLocation` (`self.Pointer`) (`KismetMathLibrary.MakeVector` _y _x) false false)
      (set `self.ClickedPostion` (`KismetMathLibrary.MakeVector2D` _locationx _locationy)))))

(event `self.Pointer.OnReleased`
  (params (TouchedComponent :type "PrimitiveComponent Object Reference") (ButtonReleased :type "Key Structure"))
  (bind (_relativelocation_x _relativelocation_y) (`KismetMathLibrary.BreakVector` (`SceneComponent.RelativeLocation` (`self.Pointer`))))
  ; OnRealease
  (`KismetSystemLibrary.PrintString` "He soltado el puntero")
  (set `self.isDraging` false)
  (bind (_y _x) (`self.CopyMousePosition`))
  (`SceneComponent.K2_AddRelativeLocation` (`self.Pointer`) (`KismetMathLibrary.MakeVector` _y _x) false false)
  (set `self.lastLocation` (`KismetMathLibrary.MakeVector2D` _relativelocation_x _relativelocation_y))
  (`self.PointerOuijaToOrigin`)
  (for _array_element (`self.combination`)
    (`KismetSystemLibrary.PrintString` _array_element))
  (`self.comprobarCombinacion`)
  (`KismetArrayLibrary.Array_Clear` (`self.combination`)))

(event `PointerOuijaToOrigin`
  (bind _originallocationpunter (`self.OriginalLocationPunter`))
  (bind (_x _y) (`KismetMathLibrary.BreakVector2D` (`self.lastLocation`)))
  ; OnRealease
  (bind (_direction _newtrack_0) (`Timeline|Timeline` :!via `PlayFromStart`)
    (:`Update`
      (`SceneComponent.K2_SetRelativeLocation` (`self.Pointer`) (`KismetMathLibrary.VLerp` (`KismetMathLibrary.MakeVector` _x _y (.z _originallocationpunter)) _originallocationpunter _newtrack_0) false false))))

(event `self.A.OnComponentBeginOverlap`
  (params (OverlappedComponent :type "PrimitiveComponent Object Reference") (OtherActor :type "Actor Object Reference") (OtherComp :type "PrimitiveComponent Object Reference") (OtherBodyIndex :type Integer) (bFromSweep :type Boolean) (SweepResult :type "HitResult Structure (by ref)"))
  ; Overlaps
  (`self.CkeckLetterUnderPointer` OtherComp "A"))

(event `comprobarCombinacion`
  ; Comprovación
  (if (!= (`KismetArrayLibrary.Array_LastIndex` (`self.combination`)) (`KismetArrayLibrary.Array_LastIndex` (`self.solution`)))
    (`KismetSystemLibrary.PrintString` "No miden ni lo mismo crack")
    (`KismetArrayLibrary.Array_Clear` (`self.combination`))
    (else
      (for (_array_element _array_index) (`self.combination`)
        (if (`KismetStringLibrary.EqualEqual_StrStr` _array_element (`|GetArrayItem` (`self.solution`) _array_index))
          (`/Engine/EditorBlueprintResources/StandardMacros.IncrementFloat` (`self.aciertos`))))
      (if (== (`self.aciertos`) 6.0)
        (`KismetSystemLibrary.PrintString` "Completado")
        (else
          (`KismetSystemLibrary.PrintString` "Palabra equivocada"))))))

(event `self.R.OnComponentBeginOverlap`
  (params (OverlappedComponent :type "PrimitiveComponent Object Reference") (OtherActor :type "Actor Object Reference") (OtherComp :type "PrimitiveComponent Object Reference") (OtherBodyIndex :type Integer) (bFromSweep :type Boolean) (SweepResult :type "HitResult Structure (by ref)"))
  ; Overlaps
  (`self.CkeckLetterUnderPointer` OtherComp "R"))

(event `self.R.OnComponentEndOverlap`
  (params (OverlappedComponent :type "PrimitiveComponent Object Reference") (OtherActor :type "Actor Object Reference") (OtherComp :type "PrimitiveComponent Object Reference") (OtherBodyIndex :type Integer))
  ; Overlaps
  (`self.InvalidateTimer` OtherComp))

(event `self.A.OnComponentEndOverlap`
  (params (OverlappedComponent :type "PrimitiveComponent Object Reference") (OtherActor :type "Actor Object Reference") (OtherComp :type "PrimitiveComponent Object Reference") (OtherBodyIndex :type Integer))
  ; Overlaps
  (`self.InvalidateTimer` OtherComp))

(event `self.C.OnComponentBeginOverlap`
  (params (OverlappedComponent :type "PrimitiveComponent Object Reference") (OtherActor :type "Actor Object Reference") (OtherComp :type "PrimitiveComponent Object Reference") (OtherBodyIndex :type Integer) (bFromSweep :type Boolean) (SweepResult :type "HitResult Structure (by ref)"))
  ; Overlaps
  (`self.CkeckLetterUnderPointer` OtherComp "C"))

(event `self.L.OnComponentBeginOverlap`
  (params (OverlappedComponent :type "PrimitiveComponent Object Reference") (OtherActor :type "Actor Object Reference") (OtherComp :type "PrimitiveComponent Object Reference") (OtherBodyIndex :type Integer) (bFromSweep :type Boolean) (SweepResult :type "HitResult Structure (by ref)"))
  ; Overlaps
  (`self.CkeckLetterUnderPointer` OtherComp "L"))

(event `Timer`
  (params (Letra :type String))
  ; Comprovación
  (bind _returnvalue (`KismetSystemLibrary.K2_SetTimerDelegate` (delegate `Añadir`) 1.0))
  (set `self.TimerVar` _returnvalue))

(event `self.C.OnComponentEndOverlap`
  (params (OverlappedComponent :type "PrimitiveComponent Object Reference") (OtherActor :type "Actor Object Reference") (OtherComp :type "PrimitiveComponent Object Reference") (OtherBodyIndex :type Integer))
  ; Overlaps
  (`self.InvalidateTimer` OtherComp))

(event `self.L.OnComponentEndOverlap`
  (params (OverlappedComponent :type "PrimitiveComponent Object Reference") (OtherActor :type "Actor Object Reference") (OtherComp :type "PrimitiveComponent Object Reference") (OtherBodyIndex :type Integer))
  ; Overlaps
  (`self.InvalidateTimer` OtherComp))

(event `Añadir`
  ; Comprovación
  (if (`KismetSystemLibrary.K2_IsValidTimerHandle` (`self.TimerVar`))
    (`KismetArrayLibrary.Array_Add` (`self.combination`) (stale `Timer` Letra))
    (`KismetSystemLibrary.PrintString` (stale `Timer` Letra))))

(event `self.S.OnComponentBeginOverlap`
  (params (OverlappedComponent :type "PrimitiveComponent Object Reference") (OtherActor :type "Actor Object Reference") (OtherComp :type "PrimitiveComponent Object Reference") (OtherBodyIndex :type Integer) (bFromSweep :type Boolean) (SweepResult :type "HitResult Structure (by ref)"))
  ; Overlaps
  (`self.CkeckLetterUnderPointer` OtherComp "S"))

(event `self.E.OnComponentBeginOverlap`
  (params (OverlappedComponent :type "PrimitiveComponent Object Reference") (OtherActor :type "Actor Object Reference") (OtherComp :type "PrimitiveComponent Object Reference") (OtherBodyIndex :type Integer) (bFromSweep :type Boolean) (SweepResult :type "HitResult Structure (by ref)"))
  ; Overlaps
  (`self.CkeckLetterUnderPointer` OtherComp "E"))

(event `self.S.OnComponentEndOverlap`
  (params (OverlappedComponent :type "PrimitiveComponent Object Reference") (OtherActor :type "Actor Object Reference") (OtherComp :type "PrimitiveComponent Object Reference") (OtherBodyIndex :type Integer))
  ; Overlaps
  (`self.InvalidateTimer` OtherComp))

(event `self.E.OnComponentEndOverlap`
  (params (OverlappedComponent :type "PrimitiveComponent Object Reference") (OtherActor :type "Actor Object Reference") (OtherComp :type "PrimitiveComponent Object Reference") (OtherBodyIndex :type Integer))
  ; Overlaps
  (`self.InvalidateTimer` OtherComp))

(event `CheckIfIsCompleted`
  (if (== (`self.PIecesPut`) 6)
    (set `self.isCompleted` true)))

(event `/Game/ProjectContent/Interfaces/I_Interact.HighLightItem`
  (`MeshComponent.SetOverlayMaterial` (`self.Marco`) "/Game/ProjectContent/Material/Ligths/M_HighLight2_Inst.M_HighLight2_Inst"))

(event `/Game/ProjectContent/Interfaces/I_Interact.StopHighLightItem`
  (`MeshComponent.SetOverlayMaterial` (`self.Marco`) null))

(fn `AddPieceToTable`
  (params (`Item Data` :type "/Game/ProjectContent/Inventory/S_Item Structure"))
  (bind (_name _description _mesh _type _collisionsize _image _itemtypedata) (break `/Game/ProjectContent/Inventory/S_Item` `Item Data`))
  (`StaticMeshComponent.SetStaticMesh` (`|GetArrayItem` (`self.Meshes`) _itemtypedata) _mesh)
  (`/Engine/EditorBlueprintResources/StandardMacros.IncrementInt` (`self.PIecesPut`)
    (:`  `
      (`self.CheckIfIsCompleted`))))

(fn `AddPointerToTable`
  (params (`Item Data` :type "/Game/ProjectContent/Inventory/S_Item Structure"))
  (`StaticMeshComponent.SetStaticMesh` (`self.Pointer`) (`.Mesh_11_32DF12CD42037715157638B0BE9178D3` (break `/Game/ProjectContent/Inventory/S_Item` `Item Data`)))
  (`/Engine/EditorBlueprintResources/StandardMacros.IncrementInt` (`self.PIecesPut`)
    (:`  `
      (`self.CheckIfIsCompleted`))))

(fn `CkeckLetterUnderPointer`
  (params (A :type "Object Object Reference") (Letra :type String))
  (if (`self.isCompleted`)
    (if (== A (`self.Box`))
      (`self.Timer` Letra))))

(fn `CopyMousePosition`
  (returns (Y :type "Float (double-precision)") (X :type "Float (double-precision)"))
  (bind (_locationx _locationy) (`PlayerController.GetMousePosition` (`GameplayStatics.GetPlayerController` 0)))
  (bind (_x _y) (`KismetMathLibrary.BreakVector2D` (/ (- (`KismetMathLibrary.MakeVector2D` _locationx _locationy) (`self.ClickedPostion`)) 33.0)))
  (return _y (* _x -1.0)))

(fn `InvalidateTimer`
  (params (A :type "Object Object Reference"))
  (if (== A (`self.Box`))
    (`KismetSystemLibrary.K2_ClearAndInvalidateTimerHandle` (`self.TimerVar`))
    (`KismetSystemLibrary.PrintString` "salio, no pongo la letra")))

(fn `UserConstructionScript`)