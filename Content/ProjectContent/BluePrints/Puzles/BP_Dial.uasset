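; BP_Dial is a clickable puzzle dial with ten positions that reports to a referenced lock.
; On BeginPlay it snaps to a random 36-degree step and derives its Number (1 to 10) from the rotation.
; Each click plays a timeline that turns it one step, ignoring clicks while it plays.
; When the turn finishes it wraps at a full circle, updates Number and calls the lock's CheckEveryTurn.
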(event `self.ReceiveBeginPlay`
  (`self.SetRandomNumber`))

(event `FindNumber`
  (set `self.Number` (- (`KismetMathLibrary.FTrunc` (/ (`self.DialRotation`) 36.0)) -1)))

(event `RotateDial`
  (if (not (`TimelineComponent.IsPlaying` (`self.DialRotation_TL`)))
    (bind (_direction _newtrack_0) (`Timeline|DialRotation_TL` :!via `PlayFromStart`)
      (:`Update`
        (bind _returnvalue (+ (`self.DialRotation`) (`KismetMathLibrary.Lerp` 0.0 36.0 _newtrack_0)))
        (`SceneComponent.K2_SetRelativeRotation` (`self.Dial`) (`KismetMathLibrary.MakeRotator` 0.0 0.0 _returnvalue) false false))
      (:`Finished`
        (set `self.DialRotation` _returnvalue)
        (if (>= (`self.DialRotation`) 360.0)
          (set `self.DialRotation` 0.0)
          (`SceneComponent.K2_SetRelativeRotation` (`self.Dial`) (`KismetMathLibrary.MakeRotator` 0.0) false false))
        (`self.FindNumber`)
        (`/Game/ProjectContent/BluePrints/Puzles/BP_CombinationLock.CheckEveryTurn` (`self.lockRef`))
        (set `self.canRotate` true)))))

(event `self.Dial.OnClicked`
  (params (TouchedComponent :type "PrimitiveComponent Object Reference") (ButtonPressed :type "Key Structure"))
  (`self.RotateDial`))

(fn `SetRandomNumber`
  (locals (LocalRotation :type "Float (double-precision)"))
  (bind _output_get (set `local.LocalRotation` (* (`KismetMathLibrary.RandomIntegerInRange` 0 9) 36)))
  (`SceneComponent.K2_SetRelativeRotation` (`self.Dial`) (`KismetMathLibrary.MakeRotator` 0.0 0.0 _output_get) false false)
  (bind _output_get_2 (set `local.LocalRotation` (`local.LocalRotation`)))
  (set `self.DialRotation` _output_get_2)
  (`self.FindNumber`))

(fn `UserConstructionScript`)