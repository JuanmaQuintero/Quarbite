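; BP_Piano is a puzzle piano whose lid (TapaPiano) opens when the player interacts with it.
; Interaction plays the OpenTape timeline to rotate the lid on roll, then marks it opened and clears its highlight.
; Highlight events set or clear an overlay material on the lid.
; It enables player input at BeginPlay, and the play-notes input only prints a placeholder string once the lid is open.
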(event `self.ReceiveBeginPlay`
  (`self.EnableInput` (`GameplayStatics.GetPlayerController` 0)))

(event `/Game/ProjectContent/Interfaces/I_Interact.Interaction`
  (params (Interactor :type "Character Object Reference") (ItemToPut :type "/Game/ProjectContent/BluePrints/Items/BP_InteractionItem Object Reference") (ComponentHit :type "ActorComponent Object Reference"))
  (bind (_direction _newtrack_0) (`Timeline|openTape`)
    (:`Update`
      (`SceneComponent.K2_SetRelativeRotation` (`self.TapaPiano`) (`KismetMathLibrary.MakeRotator` (* _newtrack_0 -150.0)) false false))
    (:`Finished`
      (set `self.isOpened` true)
      (`self.StopHighLightItem`))))

(event `/Game/ProjectContent/Interfaces/I_Interact.HighLightItem`
  (`MeshComponent.SetOverlayMaterial` (`self.TapaPiano`) "/Game/ProjectContent/Material/Ligths/M_HighLight2_Inst.M_HighLight2_Inst"))

(event `/Game/ProjectContent/Interfaces/I_Interact.StopHighLightItem`
  (`MeshComponent.SetOverlayMaterial` (`self.TapaPiano`) null))

(event `EnhancedInput|/Game/ProjectContent/Inputs/InputsPuzle/IA_PlayNotes`
  (params (ActionValue :type Boolean) (ElapsedSeconds :type "Float (double-precision)") (TriggeredSeconds :type "Float (double-precision)") (InputAction :type "InputAction Object Reference" :default "/Game/ProjectContent/Inputs/InputsPuzle/IA_PlayNotes.IA_PlayNotes"))
  (:`Started`
    (if (`self.isOpened`)
      (`KismetSystemLibrary.PrintString` "Nota"))))

(fn `UserConstructionScript`)