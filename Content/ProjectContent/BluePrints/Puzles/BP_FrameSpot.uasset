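; Picture-frame ordering puzzle where the player places, swaps or picks up BP_Frame items across three spots.
; A map keys each hit box to its attach point, expected order and current frame, and Interaction updates it as frames move between hand and spot.
; Placing into an empty spot clears the inventory entry and checks the order; swaps skip this check.
; Solving locks the puzzle, briefly shows an unlock message and updates panic duration.
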(event `self.ReceiveBeginPlay`
  ; BeginPlay
  (bind _asbp_main_character (cast `/Game/ProjectContent/BluePrints/Character/BP_MainCharacter` (`GameplayStatics.GetPlayerPawn` 0)))
  (set `self.As BP Main Character` _asbp_main_character)
  (set `self.Frame Spots` (`|MakeMap` (`self.Box1`) (make `/Game/ProjectContent/BluePrints/Puzles/ST_FrameInfo` (`self.Spot1`) 0 -1) (`self.Box`) (make `/Game/ProjectContent/BluePrints/Puzles/ST_FrameInfo` (`self.Spot2`) 1 -1) (`self.Box2`) (make `/Game/ProjectContent/BluePrints/Puzles/ST_FrameInfo` (`self.Spot3`) 2 -1) :!type "ActorComponent Object Reference")))

(event `borrar cuadro`
  (for _array_element (`/Game/ProjectContent/BluePrints/Character/BP_MainCharacter.InventaryItems` (`self.As BP Main Character`))
    (if (== (`.ItemTypeData_30_20264057492723A62849C4B967058699` (break `/Game/ProjectContent/Inventory/S_Item` _array_element)) -1)
      (`KismetArrayLibrary.Array_RemoveItem` (`/Game/ProjectContent/BluePrints/Character/BP_MainCharacter.InventaryItems` (`self.As BP Main Character`)) _array_element)
      (bind _returnvalue (`GameplayStatics.GetActorOfClass` "/Game/ProjectContent/BluePrints/Managers/BP_UIManager.BP_UIManager_C"))
      (`/Game/ProjectContent/UI/W_Menus.RefreshInventory` (`/Game/ProjectContent/BluePrints/Managers/BP_UIManager.Menus` _returnvalue)))))

(event `/Game/ProjectContent/Interfaces/I_Interact.Interaction`
  (params (Interactor :type "Character Object Reference") (ItemToPut :type "/Game/ProjectContent/BluePrints/Items/BP_InteractionItem Object Reference") (ComponentHit :type "ActorComponent Object Reference"))
  (bind _asbp_frame (cast `/Game/ProjectContent/BluePrints/Puzles/BP_Frame` ItemToPut :!pure true))
  (bind _asbp_frame_2 (cast `/Game/ProjectContent/BluePrints/Puzles/BP_Frame` ItemToPut :!pure true))
  (bind (_scenecomponent _order _currentframeorder _frame) (break `/Game/ProjectContent/BluePrints/Puzles/ST_FrameInfo` (`BlueprintMapLibrary.Map_Find` (`self.Frame Spots`) ComponentHit)))
  (bind (_scenecomponent_2 _order_2) (break `/Game/ProjectContent/BluePrints/Puzles/ST_FrameInfo` (`BlueprintMapLibrary.Map_Find` (`self.Frame Spots`) ComponentHit)))
  (bind (_scenecomponent_3 _order_3 _currentframeorder_2 _frame_2) (break `/Game/ProjectContent/BluePrints/Puzles/ST_FrameInfo` (`BlueprintMapLibrary.Map_Find` (`self.Frame Spots`) ComponentHit)))
  (if (not (`self.solved`))
    (`/Engine/EditorBlueprintResources/StandardMacros.IsValid` (`/Game/ProjectContent/BluePrints/Character/BP_MainCharacter.InLeftHand` (`self.As BP Main Character`))
      (:`Is Valid`
        (if (== _currentframeorder_2 -1)
          ; Poner
          (`BlueprintMapLibrary.Map_Add` (`self.Frame Spots`) ComponentHit (make `/Game/ProjectContent/BluePrints/Puzles/ST_FrameInfo` _scenecomponent_2 _order_2 (`/Game/ProjectContent/BluePrints/Puzles/BP_Frame.NumFrame` _asbp_frame) _asbp_frame))
          (`self.K2_AttachToComponent` ItemToPut _scenecomponent_3 " " "SnapToTarget" "SnapToTarget" "KeepWorld" true)
          (`self.borrar cuadro`)
          (set `/Game/ProjectContent/BluePrints/Character/BP_MainCharacter.InLeftHand` null (`self.As BP Main Character`))
          (set `/Game/ProjectContent/BluePrints/Character/BP_MainCharacter.HasFrame` false (`self.As BP Main Character`))
          (if (`self.CheckFramesOrder`)
            (set `self.solved` true)
            (bind _returnvalue (`GameplayStatics.GetActorOfClass` "/Game/ProjectContent/BluePrints/Managers/BP_UIManager.BP_UIManager_C"))
            (set `TextBlock.Text` "sembla que s'ha desbloquejat alguna cosa." (`/Game/ProjectContent/UI/W_Help.TextToChange` (`/Game/ProjectContent/BluePrints/Managers/BP_UIManager.Help` _returnvalue)))
            (`/Game/ProjectContent/BluePrints/Managers/BP_UIManager.Show HelpUI` _returnvalue)
            (`KismetSystemLibrary.Delay` 3.0)
            (`/Game/ProjectContent/BluePrints/Managers/BP_UIManager.Hide HelpUI` _returnvalue)
            (bind _returnvalue_2 (`GameplayStatics.GetActorOfClass` "/Game/ProjectContent/BluePrints/Managers/BP_PanicManager.BP_PanicManager_C"))
            (`/Game/ProjectContent/BluePrints/Managers/BP_PanicManager.UpdatePanicDuration` _returnvalue_2 5.0))
          (else
            ; Intercambiar
            (`self.K2_AttachToComponent` _frame_2 (`/Game/ProjectContent/BluePrints/Character/BP_MainCharacter.HoldPoint` (`self.As BP Main Character`)) "None" "SnapToTarget" "SnapToTarget" "SnapToTarget" true)
            (set `/Game/ProjectContent/BluePrints/Character/BP_MainCharacter.InLeftHand` _frame_2 (`self.As BP Main Character`))
            (`BlueprintMapLibrary.Map_Add` (`self.Frame Spots`) ComponentHit (make `/Game/ProjectContent/BluePrints/Puzles/ST_FrameInfo` _scenecomponent_3 _order_3 (`/Game/ProjectContent/BluePrints/Puzles/BP_Frame.NumFrame` _asbp_frame_2) _asbp_frame_2))
            (`self.K2_AttachToComponent` ItemToPut _scenecomponent_3 " " "SnapToTarget" "SnapToTarget" "KeepWorld" true))))
      (:`Is Not Valid`
        ; Nada en mano
        (if (!= _currentframeorder -1)
          (set `/Game/ProjectContent/BluePrints/Character/BP_MainCharacter.InLeftHand` _frame (`self.As BP Main Character`))
          (set `/Game/ProjectContent/BluePrints/Character/BP_MainCharacter.HasFrame` false (`self.As BP Main Character`))
          (`self.K2_AttachToComponent` _frame (`/Game/ProjectContent/BluePrints/Character/BP_MainCharacter.HoldPoint` (`self.As BP Main Character`)) "None" "SnapToTarget" "SnapToTarget" "SnapToTarget" true)
          (`BlueprintMapLibrary.Map_Add` (`self.Frame Spots`) ComponentHit (make `/Game/ProjectContent/BluePrints/Puzles/ST_FrameInfo` _scenecomponent _order -1 (cast `/Game/ProjectContent/BluePrints/Puzles/BP_Frame` ItemToPut :!pure true)))
          (`self.K2_AttachToComponent` (`self.Empty`) _scenecomponent " " "SnapToTarget" "SnapToTarget" "KeepWorld" true))))))

(fn `CheckFramesOrder`
  (returns (isSolved :type Boolean))
  (locals (isPuzzleSolved :type Boolean :default true))
  (bind _values (`BlueprintMapLibrary.Map_Values` (`self.Frame Spots`)))
  (for _array_element _values
    (bind (_scenecomponent _order _currentframeorder) (break `/Game/ProjectContent/BluePrints/Puzles/ST_FrameInfo` _array_element))
    (if (!= _order _currentframeorder)
      (set `local.isPuzzleSolved` false)))
  (return (`local.isPuzzleSolved`)))

(fn `UserConstructionScript`)