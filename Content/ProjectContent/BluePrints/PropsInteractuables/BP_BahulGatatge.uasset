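; Interactable garage chest whose lid opens once the level's combination lock is unlocked.
; On BeginPlay it caches the combination lock and NPC actors found by class.
; Interaction plays a small lid-movement timeline while locked, or a one-time opening timeline that then sets the NPC's forced dialogue and starts the player's dialogue.
; Highlight events toggle an overlay material on the lid.
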(event `self.ReceiveBeginPlay`
  (bind _returnvalue (`GameplayStatics.GetActorOfClass` "/Game/ProjectContent/BluePrints/Puzles/BP_CombinationLock.BP_CombinationLock_C"))
  (set `self.lock` _returnvalue)
  (bind _returnvalue_2 (`GameplayStatics.GetActorOfClass` "/Game/ProjectContent/BluePrints/NPC/BP_NPC.BP_NPC_C"))
  (set `self.NPC` _returnvalue_2))

(event `self.Interaction`
  (params (Interactor :type "Character Object Reference") (ItemToPut :type "/Game/ProjectContent/BluePrints/Items/BP_InteractionItem Object Reference") (ComponentHit :type "ActorComponent Object Reference"))
  (if (`/Game/ProjectContent/BluePrints/Puzles/BP_CombinationLock.unlucked` (`self.lock`))
    (if (not (`TimelineComponent.IsPlaying` (`self.Timeline`)))
      (`/Engine/EditorBlueprintResources/StandardMacros.DoOnce` false
        (:`Completed`
          (bind (_direction _newtrack_0) (`Timeline|Timeline` :!via `PlayFromStart`)
            (:`Update`
              (`SceneComponent.K2_SetRelativeRotation` (`self.Tapa`) (`KismetMathLibrary.MakeRotator` (* _newtrack_0 -70.0)) false false))
            (:`Finished`
              (set `/Game/ProjectContent/BluePrints/NPC/BP_NPC.forceDialogue` 3 (`self.NPC`))
              (bind _asbp_main_character (cast `/Game/ProjectContent/BluePrints/Character/BP_MainCharacter` (`GameplayStatics.GetPlayerPawn` 0)))
              (`/Game/ProjectContent/BluePrints/Character/BP_MainCharacter.Start Dialogue` _asbp_main_character "/Game/ProjectContent/Dialogues/FirstDialogue.FirstDialogue"))))))
    (else
      (bind (_direction_2 _newtrack_0_2) (`Timeline|Timeline_0` :!via `PlayFromStart`)
        (:`Update`
          (`SceneComponent.K2_SetRelativeRotation` (`self.Tapa`) (`KismetMathLibrary.MakeRotator` (* _newtrack_0_2 1.2)) false false))))))

(event `self.HighLightItem`
  (`MeshComponent.SetOverlayMaterial` (`self.Tapa`) "/Game/ProjectContent/Material/Ligths/M_HighLight2_Inst.M_HighLight2_Inst"))

(event `self.StopHighLightItem`
  (`MeshComponent.SetOverlayMaterial` (`self.Tapa`) null))

(fn `UserConstructionScript`)