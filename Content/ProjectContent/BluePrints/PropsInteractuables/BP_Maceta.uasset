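; BP_Maceta is an interactable flowerpot prop that slides along Y and back when the player interacts with it.
; BeginPlay caches the mesh's world location, and the Levantar timeline offsets Y from it, applying the result as a relative location.
; Interaction toggles the Moved flag to play the timeline forward or in reverse, ignoring input while it plays.
; Highlight events set or clear an overlay material on the mesh.
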(event `self.ReceiveBeginPlay`
  (bind (_returnvalue_x _returnvalue_y _returnvalue_z) (`KismetMathLibrary.BreakVector` (`SceneComponent.K2_GetComponentLocation` (`self.StaticMesh`))))
  (set `self.moved?` false)
  (set `self.X` _returnvalue_x)
  (set `self.Y` _returnvalue_y)
  (set `self.Z` _returnvalue_z))

(event `/Game/ProjectContent/Interfaces/I_Interact.Interaction`
  (params (Interactor :type "Character Object Reference") (ItemToPut :type "/Game/ProjectContent/BluePrints/Items/BP_InteractionItem Object Reference") (ComponentHit :type "ActorComponent Object Reference"))
  (if (not (`TimelineComponent.IsPlaying` (`self.Levantar`)))
    (if (not (`self.moved?`))
      (set `self.moved?` true)
      (bind (_direction _newtrack_0) (`Timeline|Levantar` :!via `PlayFromStart` :!label _label)
        (:`Update`
          (`SceneComponent.K2_SetRelativeLocation` (`self.StaticMesh`) (`KismetMathLibrary.MakeVector` (`self.X`) (+ (* _newtrack_0 -30.0) (`self.Y`)) (`self.Z`)) false false)))
      (else
        (set `self.moved?` false)
        (goto _label :!via `ReverseFromEnd`)))))

(event `/Game/ProjectContent/Interfaces/I_Interact.HighLightItem`
  (`MeshComponent.SetOverlayMaterial` (`self.StaticMesh`) "/Game/ProjectContent/Material/Ligths/M_HighLight2_Inst.M_HighLight2_Inst"))

(event `/Game/ProjectContent/Interfaces/I_Interact.StopHighLightItem`
  (`MeshComponent.SetOverlayMaterial` (`self.StaticMesh`) null))

(fn `UserConstructionScript`)