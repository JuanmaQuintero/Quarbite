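; BP_TapaPiano is an interactable piano lid that opens to let the player pick up an Ouija piece.
; A one-time interaction starts dialogue, forces an NPC dialogue index, blends the view to the piano and enters puzzle mode while a timeline rotates the lid.
; Input actions pick up the piece, with a help prompt shown after opening, or return the player to normal mode.
; An overlay material highlights the lid until it is opened.
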(event `EnhancedInput|/Game/ProjectContent/Inputs/InputsPuzle/IA_PickItemInside`
  (params (ActionValue :type Boolean) (ElapsedSeconds :type "Float (double-precision)") (TriggeredSeconds :type "Float (double-precision)") (InputAction :type "InputAction Object Reference" :default "/Game/ProjectContent/Inputs/InputsPuzle/IA_PickItemInside.IA_PickItemInside"))
  (:`Started`
    (if (`self.isInPiano`)
      (`/Game/ProjectContent/BluePrints/Items/BP_InteractionItem.DoPick` (`self.Ouija Piece`))
      (`/Game/ProjectContent/BluePrints/Character/BP_UIManager.Hide HelpUI` (`self.UIManager`))
      (set `self.picked` true))))

(event `self.ReceiveBeginPlay`
  (bind _asbp_main_character (cast `/Game/ProjectContent/BluePrints/Character/BP_MainCharacter` (`GameplayStatics.GetPlayerPawn` 0)))
  (set `self.Main Character` _asbp_main_character)
  (bind _returnvalue (`GameplayStatics.GetActorOfClass` "/Game/ProjectContent/BluePrints/Character/BP_UIManager.BP_UIManager_C"))
  (set `self.UIManager` _returnvalue)
  (`self.EnableInput` (`GameplayStatics.GetPlayerController` 0))
  (bind _returnvalue_2 (`GameplayStatics.GetActorOfClass` "/Game/ProjectContent/BluePrints/NPC/BP_NPC.BP_NPC_C"))
  (set `self.NPC` _returnvalue_2))

(event `EnhancedInput|/Game/ProjectContent/Inputs/InputsPuzle/IA_GoOutOfPuzzle`
  (params (ActionValue :type Boolean) (ElapsedSeconds :type "Float (double-precision)") (TriggeredSeconds :type "Float (double-precision)") (InputAction :type "InputAction Object Reference" :default "/Game/ProjectContent/Inputs/InputsPuzle/IA_GoOutOfPuzzle.IA_GoOutOfPuzzle"))
  (:`Started`
    (`PlayerController.SetViewTargetWithBlend` (`GameplayStatics.GetPlayerController` 0) (`GameplayStatics.GetPlayerPawn` 0) 1.0 "VTBlend_Linear" 0.0 false)
    (`/Game/ProjectContent/BluePrints/Character/BP_MainCharacter.goNormalMode` (`self.Main Character`))
    (`/Game/ProjectContent/BluePrints/Character/BP_UIManager.Hide HelpUI` (`self.UIManager`))
    (set `self.isInPiano` false)))

(event `/Game/ProjectContent/Interfaces/I_Interact.Interaction`
  (params (Interactor :type "Character Object Reference") (ItemToPut :type "/Game/ProjectContent/BluePrints/Items/BP_InteractionItem Object Reference") (ComponentHit :type "ActorComponent Object Reference"))
  (bind _npc (`self.NPC`))
  (bind _uimanager (`self.UIManager`))
  (`/Engine/EditorBlueprintResources/StandardMacros.DoOnce` false
    (:`Completed`
      (set `self.isInPiano` true)
      (set `/Game/ProjectContent/BluePrints/NPC/BP_NPC.forceDialogue` 2 (`self.NPC`))
      (`/Game/ProjectContent/BluePrints/Character/BP_MainCharacter.Start Dialogue` (`self.Main Character`) "/Game/ProjectContent/Dialogues/FirstDialogue.FirstDialogue")
      (set `/Game/ProjectContent/BluePrints/NPC/BP_NPC.dialogStart` (`/Game/ProjectContent/BluePrints/NPC/BP_NPC.dialogStart` _npc) _npc)
      (`PlayerController.SetViewTargetWithBlend` (`GameplayStatics.GetPlayerController` 0) self 1.0 "VTBlend_Linear" 0.0 false)
      (`/Game/ProjectContent/BluePrints/Character/BP_MainCharacter.goPuzleMode` (`self.Main Character`))
      (bind (_direction _newtrack_1) (`Timeline|Open`)
        (:`Update`
          (`SceneComponent.K2_SetRelativeRotation` (`self.Tapa`) (`KismetMathLibrary.MakeRotator` (* _newtrack_1 -90.0)) false false))
        (:`Finished`
          (if (not (`self.picked`))
            (`/Game/ProjectContent/BluePrints/Character/BP_UIManager.Show HelpUI` _uimanager)
            (set `TextBlock.Text` "Recollir objecte." (`/Game/ProjectContent/UI/W_Help.TextToChange` (`/Game/ProjectContent/BluePrints/Character/BP_UIManager.Help` _uimanager)))
            (set `self.opened` true)))))))

(event `/Game/ProjectContent/Interfaces/I_Interact.HighLightItem`
  (if (not (`self.opened`))
    (`MeshComponent.SetOverlayMaterial` (`self.Tapa`) "/Game/ProjectContent/Material/Ligths/M_HighLight2_Inst.M_HighLight2_Inst")))

(event `/Game/ProjectContent/Interfaces/I_Interact.StopHighLightItem`
  (`MeshComponent.SetOverlayMaterial` (`self.Tapa`) null))

(fn `UserConstructionScript`)