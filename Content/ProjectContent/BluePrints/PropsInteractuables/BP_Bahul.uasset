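; BP_Bahul is an interactable chest prop whose lid (Tapa) opens and closes when the player interacts with it.
; Interaction requires the cached BP_MainCharacter's CanBeginToSearch and is ignored while the timeline plays.
; A FlipFlop alternates playing and reversing that timeline, which drives the lid's relative roll.
; Highlight events set or clear an overlay material on the lid.
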(event `self.ReceiveBeginPlay`
  (bind _asbp_main_character (cast `/Game/ProjectContent/BluePrints/Character/BP_MainCharacter` (`GameplayStatics.GetPlayerPawn` 0)))
  (set `self.As BP Main Character` _asbp_main_character))

(event `/Game/ProjectContent/Interfaces/I_Interact.Interaction`
  (params (Interactor :type "Character Object Reference") (ItemToPut :type "/Game/ProjectContent/BluePrints/Items/BP_InteractionItem Object Reference") (ComponentHit :type "ActorComponent Object Reference"))
  (if (`/Game/ProjectContent/BluePrints/Character/BP_MainCharacter.canBeginToSearch` (`self.As BP Main Character`))
    (if (not (`TimelineComponent.IsPlaying` (`self.Timeline`)))
      (`/Engine/EditorBlueprintResources/StandardMacros.FlipFlop`
        (:`A`
          (bind (_direction _newtrack_0) (`Timeline|Timeline` :!via `PlayFromStart` :!label _label)
            (:`Update`
              (`SceneComponent.K2_SetRelativeRotation` (`self.Tapa`) (`KismetMathLibrary.MakeRotator` (* _newtrack_0 -70.0)) false false))))
        (:`B`
          (goto _label :!via `ReverseFromEnd`))))))

(event `/Game/ProjectContent/Interfaces/I_Interact.HighLightItem`
  (`MeshComponent.SetOverlayMaterial` (`self.Tapa`) "/Game/ProjectContent/Material/Ligths/M_HighLight2_Inst.M_HighLight2_Inst"))

(event `/Game/ProjectContent/Interfaces/I_Interact.StopHighLightItem`
  (`MeshComponent.SetOverlayMaterial` (`self.Tapa`) null))

(fn `UserConstructionScript`)