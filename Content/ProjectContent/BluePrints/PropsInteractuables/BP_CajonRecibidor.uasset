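; BP_CajonRecibidor is an interactable entrance-hall drawer prop that slides open and closed.
; Interaction alternates through a FlipFlop, playing a 2D sound and running a Timeline forward or in reverse to move the Cajon component along its local Y axis.
; Input is ignored while the Timeline plays.
; Highlight events set or clear an overlay material on the drawer.
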(event `/Game/ProjectContent/Interfaces/I_Interact.Interaction`
  (params (Interactor :type "Character Object Reference") (ItemToPut :type "/Game/ProjectContent/BluePrints/Items/BP_InteractionItem Object Reference") (ComponentHit :type "ActorComponent Object Reference"))
  (if (not (`TimelineComponent.IsPlaying` (`self.Timeline`)))
    (`/Engine/EditorBlueprintResources/StandardMacros.FlipFlop`
      (:`A`
        (`GameplayStatics.PlaySound2D` (`self.Sound1`) 1.0 1.0 0.0 null null)
        (bind (_direction _move) (`Timeline|Timeline` :!via `PlayFromStart` :!label _label)
          (:`Update`
            (`SceneComponent.K2_SetRelativeLocation` (`self.Cajon`) (`KismetMathLibrary.MakeVector` 0.0 (* _move 30.0)) false false))))
      (:`B`
        (`GameplayStatics.PlaySound2D` (`self.Sound2`) 1.0 1.0 0.0 null null)
        (goto _label :!via `ReverseFromEnd`)))))

(event `/Game/ProjectContent/Interfaces/I_Interact.HighLightItem`
  (`MeshComponent.SetOverlayMaterial` (`self.Cajon`) "/Game/ProjectContent/Material/Ligths/M_HighLight2_Inst.M_HighLight2_Inst"))

(event `/Game/ProjectContent/Interfaces/I_Interact.StopHighLightItem`
  (`MeshComponent.SetOverlayMaterial` (`self.Cajon`) null))

(fn `UserConstructionScript`)