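; Main house door interactable that stays locked until the player carries the main key gameplay tag.
; Interaction swings it open, removing the tag and a matching first-slot inventory key, or plays a slight jiggle when locked, advancing NPC dialogue in both cases.
; Once unlocked, a one-time trigger overlap saves the game at a fixed spawn, starts dialogue, enables the panic manager and reverses the timeline to close the door.
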(event `self.ReceiveBeginPlay`
  ; Begin Play
  (bind _asbp_main_character (cast `/Game/ProjectContent/BluePrints/Character/BP_MainCharacter` (`GameplayStatics.GetPlayerPawn` 0)))
  (set `self.As BP Main Character` _asbp_main_character)
  (set `self.Key` "Key")
  (`WidgetBlueprintLibrary.GetAllWidgetsOfClass` "/Game/ProjectContent/UI/W_Menus.W_Menus_C")
  (bind _returnvalue (`GameplayStatics.GetActorOfClass` "/Game/ProjectContent/BluePrints/NPC/BP_NPC.BP_NPC_C"))
  (set `self.NPC` _returnvalue))

(event `OpenDoor`
  (bind _inventaryitems (`/Game/ProjectContent/BluePrints/Character/BP_MainCharacter.InventaryItems` (`self.As BP Main Character`)))
  (bind _output (`|GetArrayItem` _inventaryitems))
  (if (`BlueprintGameplayTagLibrary.HasTag` (`/Game/ProjectContent/BluePrints/Character/BP_MainCharacter.EstatesTags` (`self.As BP Main Character`)) (struct :`TagName` "Player.HasMainKey"))
    (if (not (`TimelineComponent.IsPlaying` (`self.Timeline`)))
      (set `self.enteredHouse` true)
      (bind (_direction _newtrack_0) (`Timeline|Timeline` :!via `PlayFromStart` :!label _label)
        (:`Update`
          (`SceneComponent.K2_SetRelativeRotation` (`self.Porta`) (`KismetMathLibrary.MakeRotator` 0.0 0.0 (* _newtrack_0 90.0)) false false))
        (:`Finished`
          (`BlueprintGameplayTagLibrary.RemoveGameplayTag` (`/Game/ProjectContent/BluePrints/Character/BP_MainCharacter.EstatesTags` (`self.As BP Main Character`)) (struct :`TagName` "Player.HasMainKey"))
          (if (`KismetTextLibrary.EqualEqual_TextText` (`self.Key`) (`.Name_9_C0CB730846DD33AA88A3E9B0BD212CF4` (break `/Game/ProjectContent/Inventory/S_Item` _output)))
            (`KismetArrayLibrary.Array_RemoveItem` _inventaryitems _output)
            (`KismetSystemLibrary.PrintString` "Adios llave")
            (`/Game/ProjectContent/UI/W_Menus.RefreshInventory` (`/Game/ProjectContent/BluePrints/Character/BP_UIManager.Menus` (`/Game/ProjectContent/BluePrints/Character/BP_MainCharacter.UIManager` (`self.As BP Main Character`))))
            (set `/Game/ProjectContent/BluePrints/NPC/BP_NPC.dialogStart` 5 (`self.NPC`))))))
    (elif (not (`self.enteredHouse`))
      (`KismetSystemLibrary.PrintString` "Its Blocked, find the key")
      (bind (_direction_2 _newtrack_0_2) (`Timeline|Timeline_1` :!via `PlayFromStart`)
        (:`Update`
          (`SceneComponent.K2_SetRelativeRotation` (`self.Porta`) (`KismetMathLibrary.MakeRotator` 0.0 0.0 (* _newtrack_0_2 1.2)) false false))
        (:`Finished`
          (`/Engine/EditorBlueprintResources/StandardMacros.DoOnce` false
            (:`Completed`
              (set `/Game/ProjectContent/BluePrints/NPC/BP_NPC.dialogStart` 2 (`self.NPC`)))))))))

(event `self.Trigger.OnComponentBeginOverlap`
  (params (OverlappedComponent :type "PrimitiveComponent Object Reference") (OtherActor :type "Actor Object Reference") (OtherComp :type "PrimitiveComponent Object Reference") (OtherBodyIndex :type Integer) (bFromSweep :type Boolean) (SweepResult :type "HitResult Structure (by ref)"))
  (bind _as_bp_main_character (`self.As BP Main Character`))
  (cast `/Game/ProjectContent/BluePrints/Character/BP_MainCharacter` OtherActor)
  (if (`self.enteredHouse`)
    (`/Engine/EditorBlueprintResources/StandardMacros.DoOnce` false
      (:`Completed`
        (`/Game/ProjectContent/BluePrints/Character/BP_MainCharacter.SaveGame` _as_bp_main_character (`KismetMathLibrary.MakeTransform` (2369.450943 -961.0 88.350087)))
        (`/Game/ProjectContent/BluePrints/Character/BP_MainCharacter.Start Dialogue` _as_bp_main_character "/Game/ProjectContent/Dialogues/FirstDialogue.FirstDialogue")
        (bind _returnvalue (`GameplayStatics.GetActorOfClass` "/Game/ProjectContent/BluePrints/Managers/BP_PanicManager.BP_PanicManager_C"))
        (set `/Game/ProjectContent/BluePrints/Managers/BP_PanicManager.PanicCanAffect` true _returnvalue)
        (goto _label :!via `ReverseFromEnd`)))))

(event `/Game/ProjectContent/Interfaces/I_Interact.Interaction`
  (params (Interactor :type "Character Object Reference") (ItemToPut :type "/Game/ProjectContent/BluePrints/Items/BP_InteractionItem Object Reference") (ComponentHit :type "ActorComponent Object Reference"))
  (`self.OpenDoor`))

(fn `UserConstructionScript`)