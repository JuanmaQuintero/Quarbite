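; Movable chair prop that gets shoved by a burst of physics when its Move event fires.
; Move enables simulation on the chair, applies a strong local forward force just above its origin, then disables physics after a short delay.
; Hit only prints the hit location, throttled by a DoOnce that resets after a brief delay.
; An unconnected Push timeline holds an alternative scripted yaw-and-slide motion that never runs.
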(event `self.ReceiveBeginPlay`)

(event `Move`
  (bind _chair (`self.Chair`))
  (`PrimitiveComponent.SetSimulatePhysics` _chair true)
  (`PrimitiveComponent.AddForceAtLocationLocal` _chair (1500000.0 0.0 0.0) (0.0 0.0 15.0) "None")
  (`KismetSystemLibrary.Delay` 2.0)
  (`PrimitiveComponent.SetSimulatePhysics` (`self.Chair`) false))

(event `self.ReceiveHit`
  (params (MyComp :type "PrimitiveComponent Object Reference") (Other :type "Actor Object Reference") (OtherComp :type "PrimitiveComponent Object Reference") (bSelfMoved :type Boolean) (HitLocation :type "Vector Structure") (HitNormal :type "Vector Structure") (NormalImpulse :type "Vector Structure") (Hit :type "HitResult Structure (by ref)"))
  (`/Engine/EditorBlueprintResources/StandardMacros.DoOnce` false :!label _label
    (:`Completed`
      (`KismetSystemLibrary.PrintString` (`KismetStringLibrary.Conv_VectorToString` HitLocation))
      (`KismetSystemLibrary.Delay` 0.2)
      (goto _label :!via `Reset`))))

(fn `UserConstructionScript`)