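; BP_SaloonDoor is an interactable saloon door prop whose mesh is set from a variable in the construction script.
; On Interaction, an unclosed door plays a timeline that scales its yaw by Degrees, then marks itself Opened so it cannot replay.
; A door flagged IsClosed plays a separate, repeatable timeline scaled by DegreesClosed instead.
; Each branch ignores interaction while its timeline is playing.
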(event `/Game/ProjectContent/Interfaces/I_Interact.Interaction`
  (params (Interactor :type "Character Object Reference") (ItemToPut :type "/Game/ProjectContent/BluePrints/Items/BP_InteractionItem Object Reference") (ComponentHit :type "ActorComponent Object Reference"))
  (if (not (`self.isClosed`))
    (if (not (`TimelineComponent.IsPlaying` (`self.Timeline`)))
      (if (not (`self.opened`))
        (bind (_direction _newtrack_0) (`Timeline|Timeline` :!via `PlayFromStart`)
          (:`Update`
            (`SceneComponent.K2_SetRelativeRotation` (`self.Door`) (`KismetMathLibrary.MakeRotator` 0.0 0.0 (* _newtrack_0 (`self.Degrees`))) false false))
          (:`Finished`
            (set `self.opened` true)))))
    (elif (not (`TimelineComponent.IsPlaying` (`self.Timeline_0`)))
      (bind (_direction_2 _newtrack_0_2) (`Timeline|Timeline_0` :!via `PlayFromStart`)
        (:`Update`
          (`SceneComponent.K2_SetRelativeRotation` (`self.Door`) (`KismetMathLibrary.MakeRotator` 0.0 0.0 (* _newtrack_0_2 (`self.DegreesClosed`))) false false))))))

(fn `UserConstructionScript`
  (`StaticMeshComponent.SetStaticMesh` (`self.Door`) (`self.Mesh`)))