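; Interactable light switch that controls a linked Light actor, powered only when the BP_Fusibles puzzle is solved.
; Interaction toggles IsOn and tilts the switch mesh, updating the light's ImOn flag only once the fuses are solved.
; CheckState lights the RectLight only when both conditions hold and returns the switch state.
; The construction script finds the fuse actor and applies the initial pose; BeginPlay caches NPC and player references, unused here.
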(event `self.ReceiveBeginPlay`
  (bind _returnvalue (`GameplayStatics.GetActorOfClass` "/Game/ProjectContent/BluePrints/NPC/BP_NPC.BP_NPC_C"))
  (set `self.NPC` _returnvalue)
  (bind _asbp_main_character (cast `/Game/ProjectContent/BluePrints/Character/BP_MainCharacter` (`GameplayStatics.GetPlayerPawn` 0)))
  (set `self.Main Character` _asbp_main_character)
  (`self.CheckState`))

(event `self.Interaction`
  (params (Interactor :type "Character Object Reference") (ItemToPut :type "/Game/ProjectContent/BluePrints/Items/BP_InteractionItem Object Reference") (ComponentHit :type "ActorComponent Object Reference"))
  (`KismetSystemLibrary.PrintString` (`KismetStringLibrary.Conv_BoolToString` (`self.isOn`)))
  (bind _cangoon (`self.CheckState`))
  (if _cangoon
    (`SceneComponent.K2_SetRelativeRotation` (`self.Switch`) (`KismetMathLibrary.MakeRotator` 0.0) false false)
    (set `self.isOn` false)
    (if (`/Game/ProjectContent/BluePrints/Puzles/BP_Fusibles.solved` (`self.Fusibles`))
      (set `/Game/ProjectContent/BluePrints/Panic/BP_LuzPanic.imOn` false (`self.Light`)))
    (`self.CheckState`)
    (else
      (`SceneComponent.K2_SetRelativeRotation` (`self.Switch`) (`KismetMathLibrary.MakeRotator` 10.0) false false)
      (set `self.isOn` true)
      (if (`/Game/ProjectContent/BluePrints/Puzles/BP_Fusibles.solved` (`self.Fusibles`))
        (set `/Game/ProjectContent/BluePrints/Panic/BP_LuzPanic.imOn` true (`self.Light`)))
      (`self.CheckState`))))

(fn `CheckState`
  (returns (canGoOn :type Boolean))
  (if (and (`/Game/ProjectContent/BluePrints/Puzles/BP_Fusibles.solved` (`self.Fusibles`)) (`self.isOn`))
    (`LightComponent.SetIntensity` (`/Game/ProjectContent/BluePrints/Panic/BP_LuzPanic.RectLight` (`self.Light`)) 100000.0)
    (return true)
    (elif (and (not (`/Game/ProjectContent/BluePrints/Puzles/BP_Fusibles.solved` (`self.Fusibles`))) (`self.isOn`))
      (`LightComponent.SetIntensity` (`/Game/ProjectContent/BluePrints/Panic/BP_LuzPanic.RectLight` (`self.Light`)) 0.0)
      (return true)
      (elif (and (not (`/Game/ProjectContent/BluePrints/Puzles/BP_Fusibles.solved` (`self.Fusibles`))) (not (`self.isOn`)))
        (`LightComponent.SetIntensity` (`/Game/ProjectContent/BluePrints/Panic/BP_LuzPanic.RectLight` (`self.Light`)) 0.0)
        (return false)
        (elif (and (`/Game/ProjectContent/BluePrints/Puzles/BP_Fusibles.solved` (`self.Fusibles`)) (not (`self.isOn`)))
          (`LightComponent.SetIntensity` (`/Game/ProjectContent/BluePrints/Panic/BP_LuzPanic.RectLight` (`self.Light`)) 0.0)
          (return false))))))

(fn `UserConstructionScript`
  (bind _returnvalue (`GameplayStatics.GetActorOfClass` "/Game/ProjectContent/BluePrints/Puzles/BP_Fusibles.BP_Fusibles_C"))
  (set `self.Fusibles` _returnvalue)
  (if (`self.isOn`)
    (`SceneComponent.K2_SetRelativeRotation` (`self.Switch`) (`KismetMathLibrary.MakeRotator` 10.0) false false)
    (set `self.isOn` true)
    (else
      (`SceneComponent.K2_SetRelativeRotation` (`self.Switch`) (`KismetMathLibrary.MakeRotator` 0.0) false false)
      (set `self.isOn` false)))
  (`self.CheckState`))