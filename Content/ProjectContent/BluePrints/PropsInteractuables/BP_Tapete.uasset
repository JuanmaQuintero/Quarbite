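; BP_Tapete is an interactable rug prop that swings 90 degrees in yaw when the player interacts with it.
; Interaction alternates through a FlipFlop between playing and reversing the Mover timeline, which drives the Tapete component's relative rotation, and ignores input while the timeline plays.
; Highlight events set and clear an overlay material on the rug.
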(event `/Game/ProjectContent/Interfaces/I_Interact.Interaction`
  (params (Interactor :type "Character Object Reference") (ItemToPut :type "/Game/ProjectContent/BluePrints/Items/BP_InteractionItem Object Reference") (ComponentHit :type "ActorComponent Object Reference"))
  (if (not (`TimelineComponent.IsPlaying` (`self.Mover`)))
    (`/Engine/EditorBlueprintResources/StandardMacros.FlipFlop`
      (:`A`
        (bind (_direction _newtrack_0) (`Timeline|Mover` :!via `PlayFromStart` :!label _label)
          (:`Update`
            (`SceneComponent.K2_SetRelativeRotation` (`self.Tapete`) (`KismetMathLibrary.MakeRotator` 0.0 0.0 (* _newtrack_0 90.0)) false false))))
      (:`B`
        (goto _label :!via `ReverseFromEnd`)))))

(event `/Game/ProjectContent/Interfaces/I_Interact.HighLightItem`
  (`MeshComponent.SetOverlayMaterial` (`self.Tapete`) "/Game/ProjectContent/Material/Ligths/M_HighLight2_Inst.M_HighLight2_Inst"))

(event `/Game/ProjectContent/Interfaces/I_Interact.StopHighLightItem`
  (`MeshComponent.SetOverlayMaterial` (`self.Tapete`) null))

(fn `UserConstructionScript`)