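; BP_Doors is an interactable door prop that swings open and closed.
; Its Interaction event calls OpenDoor, which ignores requests while the Timeline is playing and otherwise alternates through a FlipFlop between playing forward and reversing.
; The Timeline track, scaled by the Degrees variable, drives the relative yaw of the Porta component.
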(event `OpenDoor`
  (if (not (`TimelineComponent.IsPlaying` (`self.Timeline`)))
    (`/Engine/EditorBlueprintResources/StandardMacros.FlipFlop`
      (:`A`
        (bind (_direction _newtrack_0) (`Timeline|Timeline` :!via `PlayFromStart` :!label _label)
          (:`Update`
            (`SceneComponent.K2_SetRelativeRotation` (`self.Porta`) (`KismetMathLibrary.MakeRotator` 0.0 0.0 (* _newtrack_0 (`self.Degrees`))) false false))))
      (:`B`
        (goto _label :!via `ReverseFromEnd`)))))

(event `self.Interaction`
  (params (Interactor :type "Character Object Reference") (ItemToPut :type "/Game/ProjectContent/BluePrints/Items/BP_InteractionItem Object Reference") (ComponentHit :type "ActorComponent Object Reference"))
  (`self.OpenDoor`))

(fn `UserConstructionScript`)