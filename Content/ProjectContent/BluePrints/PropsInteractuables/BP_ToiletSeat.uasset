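; BP_ToiletSeat is an interactable toilet prop whose lid (Tapa) can be animated downward.
; BeginPlay caches the lid's relative rotation.
; The Bajartapa event plays the Bajar timeline, whose track scales a -90 degree roll offset added to the cached roll.
; Each update sets pitch and yaw to zero, so their cached values go unused.
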(event `self.ReceiveBeginPlay`
  (set `self.X (Roll)` (.roll (`SceneComponent.RelativeRotation` (`self.Tapa`))))
  (set `self.Y (Pitch)` (.pitch (`SceneComponent.RelativeRotation` (`self.Tapa`))))
  (set `self.Z (Yaw)` (.yaw (`SceneComponent.RelativeRotation` (`self.Tapa`)))))

(event `Bajartapa`
  (bind (_direction _newtrack_0) (`Timeline|bajar`)
    (:`Update`
      (`SceneComponent.K2_SetRelativeRotation` (`self.Tapa`) (`KismetMathLibrary.MakeRotator` (+ (* _newtrack_0 -90.0) (`self.X (Roll)`))) false false))))

(fn `UserConstructionScript`)