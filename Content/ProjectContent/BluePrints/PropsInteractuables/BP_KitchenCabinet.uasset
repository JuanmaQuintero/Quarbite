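; Interactable kitchen cabinet whose door stays locked until the level's BP_FrameSpot puzzle is solved.
; On BeginPlay it caches the BP_FrameSpot and BP_UIManager actors.
; When solved, interaction alternates opening and closing via a FlipFlop and a timeline driving door yaw, with sounds, ignoring input while it plays.
; While locked, it shows a Spanish hint through the UI manager for a few seconds; the construction script assigns the door mesh.
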(event `self.ReceiveBeginPlay`
  (bind _returnvalue (`GameplayStatics.GetActorOfClass` "/Game/ProjectContent/BluePrints/Puzles/BP_FrameSpot.BP_FrameSpot_C"))
  (set `self.frames` _returnvalue)
  (bind _returnvalue_2 (`GameplayStatics.GetActorOfClass` "/Game/ProjectContent/BluePrints/Managers/BP_UIManager.BP_UIManager_C"))
  (set `self.UIManager` _returnvalue_2))

(event `/Game/ProjectContent/Interfaces/I_Interact.Interaction`
  (params (Interactor :type "Character Object Reference") (ItemToPut :type "/Game/ProjectContent/BluePrints/Items/BP_InteractionItem Object Reference") (ComponentHit :type "ActorComponent Object Reference"))
  (bind _uimanager (`self.UIManager`))
  (if (`/Game/ProjectContent/BluePrints/Puzles/BP_FrameSpot.solved` (`self.frames`))
    (if (not (`TimelineComponent.IsPlaying` (`self.open/close`)))
      (`/Engine/EditorBlueprintResources/StandardMacros.FlipFlop`
        (:`A`
          (`GameplayStatics.PlaySound2D` "/Game/ProjectContent/Music/SE/Armari/openArmari1.openArmari1" 1.0 1.0 0.0 null null)
          (bind (_direction _newtrack_0) (`Timeline|open/close` :!via `PlayFromStart` :!label _label)
            (:`Update`
              (`SceneComponent.K2_SetRelativeRotation` (`self.Door`) (`KismetMathLibrary.MakeRotator` 0.0 0.0 (* _newtrack_0 (`self.Degrees`))) false false))))
        (:`B`
          (`GameplayStatics.PlaySound2D` "/Game/ProjectContent/Music/SE/Armari/openArmari3.openArmari3" 1.0 1.0 0.0 null null)
          (goto _label :!via `ReverseFromEnd`))))
    (else
      (set `TextBlock.Text` "Esta bloqueado, porque será?" (`/Game/ProjectContent/UI/W_Help.TextToChange` (`/Game/ProjectContent/BluePrints/Managers/BP_UIManager.Help` _uimanager)))
      (`/Game/ProjectContent/BluePrints/Managers/BP_UIManager.Show HelpUI` _uimanager)
      (`KismetSystemLibrary.Delay` 3.0)
      (`/Game/ProjectContent/BluePrints/Managers/BP_UIManager.Hide HelpUI` _uimanager))))

(fn `UserConstructionScript`
  (`StaticMeshComponent.SetStaticMesh` (`self.Door`) (`self.Mesh`)))