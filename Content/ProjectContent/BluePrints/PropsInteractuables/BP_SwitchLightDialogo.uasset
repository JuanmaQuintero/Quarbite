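; BP_SwitchLightDialogo is an interactable light switch that triggers dialogue and toggles a rect light.
; On BeginPlay it caches the BP_NPC and the player's BP_MainCharacter.
; While IsFirstTime is set, Interaction changes the NPC's DialogStart and starts FirstDialogue on the interacting character; this graph never clears that flag.
; Otherwise a FlipFlop alternates light intensity on and off, checking CanTurnOnLights after each flip, so blocked presses still advance it.
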(event `self.ReceiveBeginPlay`
  (bind _returnvalue (`GameplayStatics.GetActorOfClass` "/Game/ProjectContent/BluePrints/NPC/BP_NPC.BP_NPC_C"))
  (set `self.NPC` _returnvalue)
  (bind _asbp_main_character (cast `/Game/ProjectContent/BluePrints/Character/BP_MainCharacter` (`GameplayStatics.GetPlayerPawn` 0)))
  (set `self.Main Character` _asbp_main_character))

(event `/Game/ProjectContent/Interfaces/I_Interact.Interaction`
  (params (Interactor :type "Character Object Reference") (ItemToPut :type "/Game/ProjectContent/BluePrints/Items/BP_InteractionItem Object Reference") (ComponentHit :type "ActorComponent Object Reference"))
  (if (`self.isFirstTime`)
    (set `/Game/ProjectContent/BluePrints/NPC/BP_NPC.dialogStart` 7 (`self.NPC`))
    (bind _asbp_main_character (cast `/Game/ProjectContent/BluePrints/Character/BP_MainCharacter` Interactor))
    (`/Game/ProjectContent/BluePrints/Character/BP_MainCharacter.Start Dialogue` _asbp_main_character "/Game/ProjectContent/Dialogues/FirstDialogue.FirstDialogue")
    (else
      (`/Engine/EditorBlueprintResources/StandardMacros.FlipFlop`
        (:`A`
          (if (`/Game/ProjectContent/BluePrints/Character/BP_MainCharacter.canTurnOnLights` (`self.Main Character`))
            (`LightComponent.SetIntensity` (`RectLight.RectLightComponent` (`self.Light`)) 200.0)))
        (:`B`
          (if (`/Game/ProjectContent/BluePrints/Character/BP_MainCharacter.canTurnOnLights` (`self.Main Character`))
            (`LightComponent.SetIntensity` (`RectLight.RectLightComponent` (`self.Light`)) 0.0)))))))

(fn `UserConstructionScript`)