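; BP_PuertaPadres is the parents' door, which can slam shut once and then be opened by interaction.
; BeginPlay caches the door's world rotation, and Portazo uses a DoOnce and the Cerrar timeline to swing its relative yaw from that cached yaw, then flags it closed.
; Interaction works only once that flag is set, playing a second timeline that swings the yaw the opposite way from zero.
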(event `self.ReceiveBeginPlay`
  (set `self.X (Roll)` (.roll (`SceneComponent.K2_GetComponentRotation` (`self.Door`))))
  (set `self.Y (Pitch)` (.pitch (`SceneComponent.K2_GetComponentRotation` (`self.Door`))))
  (set `self.Z (Yaw)` (.yaw (`SceneComponent.K2_GetComponentRotation` (`self.Door`)))))

(event `Portazo`
  (`/Engine/EditorBlueprintResources/StandardMacros.DoOnce` false
    (:`Completed`
      (bind (_direction _newtrack_0) (`Timeline|Cerrar` :!via `PlayFromStart`)
        (:`Update`
          (`SceneComponent.K2_SetRelativeRotation` (`self.Door`) (`KismetMathLibrary.MakeRotator` 0.0 0.0 (+ (* _newtrack_0 130.0) (`self.Z (Yaw)`))) false false))
        (:`Finished`
          (set `self.isClosed` true))))))

(event `/Game/ProjectContent/Interfaces/I_Interact.Interaction`
  (params (Interactor :type "Character Object Reference") (ItemToPut :type "/Game/ProjectContent/BluePrints/Items/BP_InteractionItem Object Reference") (ComponentHit :type "ActorComponent Object Reference"))
  (if (`self.isClosed`)
    (bind (_direction _newtrack_0) (`Timeline|Timeline` :!via `PlayFromStart`)
      (:`Update`
        (`SceneComponent.K2_SetRelativeRotation` (`self.Door`) (`KismetMathLibrary.MakeRotator` 0.0 0.0 (* _newtrack_0 -130.0)) false false)))))

(fn `UserConstructionScript`)