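; BP_LuzProba is a placed actor, apparently a test light, that switches panic off while the player is near it.
; Each tick it checks 2D distance to BP_MainCharacter and calls PanicOff or PanicOn on BP_PanicManager when crossing a threshold.
; Separate inner and outer thresholds add hysteresis so the state does not flicker at the boundary.
; The construction script draws a debug sphere at the inner radius.
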(event `self.ReceiveBeginPlay`
  (bind _asbp_main_character (cast `/Game/ProjectContent/BluePrints/Character/BP_MainCharacter` (`GameplayStatics.GetPlayerCharacter` 0)))
  (set `self.As BP Main Character` _asbp_main_character)
  (set `self.currentThreshold` (`self.innerThresholdDistance`))
  (bind _returnvalue (`GameplayStatics.GetActorOfClass` "/Game/ProjectContent/BluePrints/Managers/BP_PanicManager.BP_PanicManager_C"))
  (set `self.PanicManager` _returnvalue))

(event `self.ReceiveTick`
  (params (DeltaSeconds :type "Float (single-precision)"))
  (if (< (`KismetMathLibrary.Vector_Distance2D` (`self.K2_GetActorLocation`) (`self.K2_GetActorLocation` (`self.As BP Main Character`))) (`self.currentThreshold`))
    (if (not (`self.transitioned`))
      (set `self.transitioned` true)
      (set `self.currentThreshold` (`self.outterThresholdDistance`))
      (`/Game/ProjectContent/BluePrints/Managers/BP_PanicManager.PanicOff` (`self.PanicManager`))
      (`KismetSystemLibrary.PrintString` "Hello"))
    (elif (`self.transitioned`)
      (set `self.transitioned` false)
      (set `self.currentThreshold` (`self.innerThresholdDistance`))
      (`/Game/ProjectContent/BluePrints/Managers/BP_PanicManager.PanicOn` (`self.PanicManager`)))))

(fn `UserConstructionScript`
  (`KismetSystemLibrary.DrawDebugSphere` (`self.K2_GetActorLocation`) (`self.innerThresholdDistance`) 12 (struct :`R` 1.0 :`G` 1.0 :`B` 1.0 :`A` 1.0) 1.0 1.0))