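; Pickup actor for an item defined by a row in the DT_Items data table, selected by its Name variable.
; The construction script looks up that row and applies its mesh to the Item component.
; On Interaction it prints a debug string, then DoPick re-reads the row, disables Box collision and passes the item data and a self-reference to the player pawn through PickUpItemMessage.
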(event `/Game/ProjectContent/Interfaces/I_Interact.Interaction`
  (params (Interactor :type "Character Object Reference"))
  (`KismetSystemLibrary.PrintString` "Picked")
  (`self.DoPick`))

(fn `DoPick`
  (bind _returnvalue (`|GetDataTableRow` "/Game/ProjectContent/Inventory/DT_Items.DT_Items" (`self.name`))
    (:`then`
      (`PrimitiveComponent.SetCollisionEnabled` (`self.Box`) "NoCollision")
      (message `/Game/ProjectContent/Interfaces/I_Interact.PickUpItem` (`GameplayStatics.GetPlayerPawn` 0) _returnvalue self))))

(fn `UserConstructionScript`
  (bind _returnvalue (`|GetDataTableRow` "/Game/ProjectContent/Inventory/DT_Items.DT_Items" (`self.name`))
    (:`then`
      (`StaticMeshComponent.SetStaticMesh` (`self.Item`) (`.Mesh_11_32DF12CD42037715157638B0BE9178D3` (break `/Game/ProjectContent/Inventory/S_Item` _returnvalue))))))