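; BP_InteractionItem is a pickup item whose mesh and collision box size come from a DT_Items row looked up by Name in the construction script.
; Interaction looks up the row again, stores it, disables box collision and sends the data and a self reference to the player pawn through PickUpItemMessage.
; Highlight events set or clear an overlay material on the mesh.
; The DestroyActor node in DoPick never runs.
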(event `/Game/ProjectContent/Interfaces/I_Interact.Interaction`
  (params (Interactor :type "Character Object Reference") (ItemToPut :type "/Game/ProjectContent/BluePrints/Items/BP_InteractionItem Object Reference") (ComponentHit :type "ActorComponent Object Reference"))
  (`KismetSystemLibrary.PrintString` "Picked")
  (`self.DoPick`))

(event `/Game/ProjectContent/Interfaces/I_Interact.HighLightItem`
  (`MeshComponent.SetOverlayMaterial` (`self.Item`) "/Game/ProjectContent/Material/Ligths/M_HighLight2_Inst.M_HighLight2_Inst"))

(event `/Game/ProjectContent/Interfaces/I_Interact.StopHighLightItem`
  (`MeshComponent.SetOverlayMaterial` (`self.Item`) null))

(fn `DoPick`
  (bind _returnvalue (`|GetDataTableRow` "/Game/ProjectContent/Inventory/DT_Items.DT_Items" (`self.name`))
    (:`then`
      (set `self.ItemData` _returnvalue)
      (`PrimitiveComponent.SetCollisionEnabled` (`self.Box`) "NoCollision")
      (message `/Game/ProjectContent/Interfaces/I_Interact.PickUpItem` (`GameplayStatics.GetPlayerPawn` 0) _returnvalue self))))

(fn `UserConstructionScript`
  (bind _returnvalue (`|GetDataTableRow` "/Game/ProjectContent/Inventory/DT_Items.DT_Items" (`self.name`))
    (:`then`
      (bind (_name _description _mesh _type _collisionsize) (break `/Game/ProjectContent/Inventory/S_Item` _returnvalue))
      (`StaticMeshComponent.SetStaticMesh` (`self.Item`) _mesh)
      (`BoxComponent.SetBoxExtent` (`self.Box`) _collisionsize true))))