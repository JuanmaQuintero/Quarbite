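; BP_Letter is a pickable letter item that shows its content on screen when the player interacts with it.
; It finds BP_UIManager on BeginPlay and runs the parent's pick logic on interaction.
; It then switches BP_MainCharacter into puzzle mode, has the UI manager show the letter panel filled with the ItemData image, and destroys itself.
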(event `self.ReceiveBeginPlay`
  (bind _returnvalue (`GameplayStatics.GetActorOfClass` "/Game/ProjectContent/BluePrints/Character/BP_UIManager.BP_UIManager_C"))
  (set `self.UIManager` _returnvalue))

(event `/Game/ProjectContent/Interfaces/I_Interact.Interaction`
  (params (Interactor :type "Character Object Reference") (ItemToPut :type "/Game/ProjectContent/BluePrints/Items/BP_InteractionItem Object Reference") (ComponentHit :type "ActorComponent Object Reference"))
  (bind _uimanager (`self.UIManager`))
  (`self.DoPick`)
  (bind _asbp_main_character (cast `/Game/ProjectContent/BluePrints/Character/BP_MainCharacter` (`GameplayStatics.GetPlayerPawn` 0)))
  (`/Game/ProjectContent/BluePrints/Character/BP_MainCharacter.goPuzleMode` _asbp_main_character)
  (`/Game/ProjectContent/BluePrints/Character/BP_UIManager.ShowLetterContent` _uimanager)
  (`Image.SetBrushFromTexture` (`/Game/ProjectContent/UI/W_Letters.Content` (`/Game/ProjectContent/BluePrints/Character/BP_UIManager.Letters` _uimanager)) (`.Image_27_AA013B034816250D1E8E73AEF692F6AF` (break `/Game/ProjectContent/Inventory/S_Item` (`self.ItemData`))) false)
  (`self.K2_DestroyActor`))

(fn `DoPick`
  (`parent.DoPick`))

(fn `UserConstructionScript`
  (`parent.UserConstructionScript`))